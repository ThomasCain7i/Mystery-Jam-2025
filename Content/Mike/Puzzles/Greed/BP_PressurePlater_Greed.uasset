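; Pressure plate for the Greed puzzle that detects the player or the key item, depending on its plate type flags, and reports to BPGreed.
; Box overlaps track both states, sending player changes immediately.
; The first movable-tagged overlap starts a looping timer that reports the key item as placed only if no more than one greed item overlaps.
; The puzzle-complete dispatcher from BPGreed clears that timer.
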(event OnComponentBeginOverlap(BoxCollider)
  (params (OverlappedComponent :type Primitive%20Component%20Object%20Reference) (OtherActor :type Actor%20Object%20Reference) (OtherComp :type Primitive%20Component%20Object%20Reference) (OtherBodyIndex :type Integer) (bFromSweep :type Boolean) (SweepResult :type Hit%20Result%20Structure%20%28by%20ref%29))
  (Utilities|FlowControl|Sequence
    (:then_0
      ;[1 1 1] Start Timer Handle
      (if (and (Components|ComponentHasTag OtherComp (Variables|Collision|Tag|GetMovableTag)) (not (Variables|States|GetbTimerStarted)))
        (Variables|States|SetbTimerStarted true)
        (CallFunction|CallCheckItemsonPlate)))
    (:then_1
      ;[1 1 1] Set If key item on the plate
      (if (and (Actor|ActorHasTag OtherActor (Variables|Collision|Tag|GetGreedKeyItemTag)) (Variables|ClassSettings|GetbIsKeyItemPlate))
        (Variables|Collision|Plates|SetbGreedkeyItemOnPlate true)))
    (:then_2
      ;[1 1 1] Set Is player on the plate
      (if (and (Actor|ActorHasTag OtherActor (Variables|Collision|Tag|GetPlayerTag)) (Variables|ClassSettings|GetbIsPlayerPlate))
        (bind _output_get (Variables|Collision|Plates|SetbIsPlayerOnPlate true))
        (Default|UpdateGreedPlatePlayer (Variables|ClassSettings|GetBP_Greed) _output_get)))))

(event OnComponentEndOverlap(BoxCollider)
  (params (OverlappedComponent :type Primitive%20Component%20Object%20Reference) (OtherActor :type Actor%20Object%20Reference) (OtherComp :type Primitive%20Component%20Object%20Reference) (OtherBodyIndex :type Integer))
  ;[1 1 1] End overlap
  (Utilities|FlowControl|Sequence
    (:then_0
      (if (and (Actor|ActorHasTag OtherActor (Variables|Collision|Tag|GetGreedKeyItemTag)) (Variables|ClassSettings|GetbIsKeyItemPlate))
        (Variables|Collision|Plates|SetbGreedkeyItemOnPlate false)))
    (:then_1
      (if (and (Actor|ActorHasTag OtherActor (Variables|Collision|Tag|GetPlayerTag)) (Variables|ClassSettings|GetbIsPlayerPlate))
        (bind _output_get (Variables|Collision|Plates|SetbIsPlayerOnPlate false))
        (Default|UpdateGreedPlatePlayer (Variables|ClassSettings|GetBP_Greed) _output_get)))))

(event Custom|CallCheckItemsOnPlate
  ;[1 1 1] Start Timer
  (if (not (Variables|States|GetbPuzzleComplete))
    (bind _returnvalue (Utilities|Time|SetTimerbyEvent (EventDispatchers|CreateEvent :!event Custom|CheckItemsOnPlate) 1.0 true))
    (Variables|Collision|Plates|SetCheckTimerHandle _returnvalue)))

(event Custom|CheckItemsOnPlate
  (bind _bgreedkeyitemonplate (Variables|Collision|Plates|GetbGreedkeyItemOnPlate))
  (bind _bp_greed (Variables|ClassSettings|GetBP_Greed))
  ;[1 1 1] Timer Handle
  (if (> (Utilities|Array|Length (Collision|GetOverlappingActors (Variables|Default|GetBoxCollider) "/Game/Mike/Puzzles/Greed/BP_GreedItem_Base.BP_GreedItem_Base_C" :!class /Script/Engine.PrimitiveComponent)) 1)
    (Default|UpdateGreedPlateKeyItem _bp_greed false)
    (elif _bgreedkeyitemonplate
      (Default|UpdateGreedPlateKeyItem _bp_greed _bgreedkeyitemonplate)
      (else
        (Default|UpdateGreedPlateKeyItem _bp_greed false)))))

(event Custom|OnGreedPuzzleComplete_Event
  (bind _checktimerhandle (Variables|Collision|Plates|GetCheckTimerHandle))
  ;[1 1 1] On Begin Play
  (Variables|States|SetbPuzzleComplete true)
  (if (Utilities|Time|IsValidTimerHandle _checktimerhandle)
    (Utilities|Time|ClearandInvalidateTimerbyHandle _checktimerhandle)
    (Development|PrintString "Pressure plates stop working")))

(event EventBeginPlay
  ;[1 1 1] On Begin Play
  (EventDispatchers|AssignOnGreedPuzzleComplete (Variables|ClassSettings|GetBP_Greed) (delegate Custom|OnGreedPuzzleComplete_Event)))

(fn ConstructionScript)