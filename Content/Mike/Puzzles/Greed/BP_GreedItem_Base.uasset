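; BP_GreedItem_Base is the base item Blueprint for the Greed puzzle, configured from a data table row.
; On BeginPlay it looks up its GreedItemData row handle and sets its static mesh from that row, scaled by UpdateVisualsScale.
; Rows flagged as key items replace the Tags array with KeyItemTag.
; The construction script is empty, so these changes apply only at runtime.
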(event EventBeginPlay
  (bind _greeditemdata (Variables|Default|GetGreedItemData))
  (bind _staticmesh (Variables|Default|GetStaticMesh))
  (bind _returnvalue (Utilities|GetDataTableRow (.datatable _greeditemdata) (.rowname _greeditemdata))
    (:then
      (if (.bIsKeyItem (Utilities|Struct|BreakST_GreedItems _returnvalue))
        (Variables|Default|SetTags (Utilities|Array|MakeArray (Variables|Default|GetKeyItemTag))))
      (Components|StaticMesh|SetStaticMesh _staticmesh (.StaticMesh (Utilities|Struct|BreakST_GreedItems _returnvalue)))
      (Transformation|SetWorldScale3D _staticmesh (Variables|Default|GetUpdateVisualsScale)))))

(fn ConstructionScript)