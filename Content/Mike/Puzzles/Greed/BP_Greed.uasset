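; BP_Greed is the Greed puzzle actor, completed when both the player and a key item are on the plates.
; Interface events store the player and key item plate states, and each update re-checks both.
; When both are true, it calls the OnGreedPuzzleComplete dispatcher, prints a debug message and activates a particle system.
; Nothing latches completion, so it can fire again on later updates.
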(event Custom|CheckBothPlates
  ;[1 1 1] Check both player and key item is on the platform
  (if (and (Variables|Default|GetbPlayerOnPlate) (Variables|Default|GetbKeyItemOnPlate))
    (Default|CallOnGreedPuzzleComplete)
    (Development|PrintString "Puzzle Complete " true true "(R=0.000000,G=1.000000,B=0.007945,A=1.000000)" 1e+01)
    (Components|Activation|Activate (Variables|Default|GetParticleSystem) false)))

(event EventUpdateGreedPlateKeyItem
  (params (bIsKeyItemOnPlate :type Boolean))
  ;[1 1 1] Interfaces
  (Variables|Default|SetbKeyItemOnPlate bIsKeyItemOnPlate)
  (Development|PrintString "Geed plate : Key item on plate" true true "(R=0.501961,G=0.090196,B=1.000000,A=1.000000)" 5.0)
  (CallFunction|CheckBothPlates))

(event EventUpdateGreedPlatePlayer
  (params (bIsPlayerOnPlate :type Boolean))
  ;[1 1 1] Interfaces
  (Variables|Default|SetbPlayerOnPlate bIsPlayerOnPlate)
  (Development|PrintString "Greed plate : player on plate " true true "(R=0.501961,G=0.090196,B=1.000000,A=1.000000)" 5.0)
  (CallFunction|CheckBothPlates))

(fn ConstructionScript)