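; Manager actor for the Gluttony puzzle that checks whether every food plate in its area holds the goal weight.
; A looping timer runs a debug-drawn box trace to gather unique BP_FoodPlate actors and counts those weighing GoalWeight plus one.
; When all found plates match, it calls GluttonyPuzzleCompleted, clears the timer and destroys itself.
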(event Custom|CheckAllPlatesWeight
  (bind _self self)
  (bind _as_bp_food_plate (Variables|Collision|GetAs%20BP%20Food%20Plate))
  (bind _defaultsceneroot (Variables|Default|GetDefaultSceneRoot _self))
  (bind _returnvalue (Transformation|GetWorldLocation _defaultsceneroot))
  (Development|PrintString "Check all plates")
  (if (not (Variables|Outcome|GetbPuzzleCompleted))
    ;[1 1 1] Get all the weights from each plate
    (Variables|Outcome|SetPlatesWithCorrectWeight 0)
    (Utilities|Array|Clear (Variables|Collision|GetAs%20BP%20Food%20Plate))
    (bind (_outhits _returnvalue_2) (Class|KismetSystemLibrary|BoxTraceMultiforObjects _returnvalue (+ _returnvalue "1.000000,1.000000,1.000000") (Variables|Collision|GetHalf%20Size) "0, 0, 0" (Variables|Collision|GetObject%20Types) false (Utilities|Array|MakeArray self) "ForDuration" true "(R=1.000000,G=0.329115,B=0.931142,A=1.000000)" "(R=0.527988,G=0.968142,B=1.000000,A=1.000000)" 2.0))
    (if _returnvalue_2
      (for _array_element _outhits
        (bind _asbp_food_plate (Utilities|Casting|CastToBP_FoodPlate (.HitActor (Collision|BreakHitResult _array_element))))
        (Utilities|Array|AddUnique (Variables|Collision|GetAs%20BP%20Food%20Plate) _asbp_food_plate))
      (Variables|Outcome|SetTotalPlates (Utilities|Array|Length _as_bp_food_plate))
      (for _array_element_2 _as_bp_food_plate
        (bind _totalweight (Default|CheckPlateWeight _array_element_2))
        (Development|PrintString (Utilities|String|Append (Utilities|GetDisplayName _array_element_2) " = " (Utilities|String|ToString(Integer) _totalweight)) true true "(R=1.000000,G=0.579586,B=0.101651,A=1.000000)" 3.0)
        (if (== _totalweight (+ (Variables|Outcome|GetGoalWeight) 1))
          (Math|Integer|IncrementInt (Variables|Outcome|GetPlatesWithCorrectWeight))))
      (CallFunction|CheckifPassed))))

(event Custom|CheckIfPassed
  ;[1 1 1] Pass or fail the puzzle
  (if (== (Variables|Outcome|GetTotalPlates) (Variables|Outcome|GetPlatesWithCorrectWeight))
    (CallFunction|OnPuzzleCompleted)
    (Development|PrintString "Puzzle Complete" true true "(R=0.000000,G=1.000000,B=0.066155,A=1.000000)" 5.0)
    (else
      (Variables|Outcome|SetbPuzzleCompleted false)
      (Development|PrintString "Puzzle Failed" true true "(R=1.000000,G=0.166591,B=0.000000,A=1.000000)" 5.0))))

(event Custom|OnPuzzleCompleted
  (bind _checkallplatewieighstimer (Variables|Timer|GetCheckAllPlateWieighsTimer))
  ;[0.05989 1 0.01696] Puzzle is completed
  (Variables|Outcome|SetbPuzzleCompleted true)
  (Default|CallGluttonyPuzzleCompleted)
  (if (Utilities|Time|IsValidTimerHandle _checkallplatewieighstimer)
    (Utilities|Time|ClearandInvalidateTimerbyHandle _checkallplatewieighstimer)
    (Actor|DestroyActor)))

(event EventBeginPlay
  ;[1 1 1] Comment
  (bind _returnvalue (Utilities|Time|SetTimerbyEvent (delegate Custom|CheckAllPlatesWeight) (Variables|Timer|GetLoopTime) true 1.0))
  (Variables|Timer|SetCheckAllPlateWieighsTimer _returnvalue))

(fn ConstructionScript)