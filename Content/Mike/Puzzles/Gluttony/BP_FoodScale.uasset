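; Balance scale for the Gluttony puzzle that tips according to the food weight on its two plates.
; A one-second looping timer totals BPC_ItemHasWeight weights of BP_Food_Base actors overlapping each plate collider.
; MoveScale then snaps the Plates pitch to level or either tilt.
; An IsMoving flag gates checks, with a loop-count fallback if it sticks, and OnPuzzleComplete clears the timer.
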(event Custom|UpdateLeftSideScale
  ;[1 1 1] Update Left side scale
  (Variables|Default|SetbIsMoving true)
  (Variables|Default|SetLeftSideCurrentWeight 0)
  (for _array_element (Collision|GetOverlappingActors (Variables|Default|GetLeftPlateCollider) "/Game/Mike/Puzzles/Gluttony/BP_Food_Base.BP_Food_Base_C" :!class /Script/Engine.PrimitiveComponent)
    (Utilities|IsValid (Actor|GetComponentbyClass _array_element "/Game/Mike/Puzzles/Gluttony/BPC_ItemHasWeight.BPC_ItemHasWeight_C")
      (:Is%20Valid
        (bind _weight (Default|GetItemWeight (Actor|GetComponentbyClass _array_element "/Game/Mike/Puzzles/Gluttony/BPC_ItemHasWeight.BPC_ItemHasWeight_C")))
        (bind _output_get (Variables|Default|SetLeftSideCurrentWeight (+ _weight (Variables|Default|GetLeftSideCurrentWeight))))
        (Development|PrintString (Utilities|String|ToString(Integer) _output_get) true true "(R=0.000000,G=0.660000,B=1.000000,A=1.000000)" 1.0)))))

(event Custom|UpdateRightSideScale
  ;[1 1 1] Update Right side of scale
  (Variables|Default|SetbIsMoving true)
  (Variables|Default|SetRightSideCurrentWeight 0)
  (for _array_element (Collision|GetOverlappingActors (Variables|Default|GetRightPlateCollider) "/Game/Mike/Puzzles/Gluttony/BP_Food_Base.BP_Food_Base_C" :!class /Script/Engine.PrimitiveComponent)
    (Utilities|IsValid (Actor|GetComponentbyClass _array_element "/Game/Mike/Puzzles/Gluttony/BPC_ItemHasWeight.BPC_ItemHasWeight_C")
      (:Is%20Valid
        (bind _weight (Default|GetItemWeight (Actor|GetComponentbyClass _array_element "/Game/Mike/Puzzles/Gluttony/BPC_ItemHasWeight.BPC_ItemHasWeight_C")))
        (bind _output_get (Variables|Default|SetRightSideCurrentWeight (+ _weight (Variables|Default|GetRightSideCurrentWeight))))
        (Development|PrintString (Utilities|String|ToString(Integer) _output_get) true true "(R=1.000000,G=0.234955,B=0.947431,A=1.000000)" 1.0)))))

(event Custom|CheckScaleWeights
  ;[1 1 1] Timer Logic
  (if (Variables|Default|GetbIsMoving)
    ;[1 1 1] Manually reset is moving bool, sometimes get stuck
    (if (not (>= (Variables|Default|GetCurrentLoops) (Variables|Default|GetLoopsBeforeManualReset)))
      (Math|Integer|IncrementInt (Variables|Default|GetCurrentLoops)
        (:%20%20
          (Development|PrintString "Currently Moving")))
      (else
        (Variables|Default|SetbIsMoving false)))
    (else
      (Variables|Default|SetCurrentLoops 0)
      (Utilities|FlowControl|Sequence
        (:then_0
          (CallFunction|UpdateLeftSideScale))
        (:then_1
          (CallFunction|UpdateRightSideScale))
        (:then_2
          (CallFunction|MoveScale))
        (:then_3
          (Utilities|FlowControl|Delay 0.5)
          (Variables|Default|SetbIsMoving false))))))

(event EventBeginPlay
  ;[1 1 1] Begin Play
  (bind _returnvalue (Utilities|Time|SetTimerbyEvent (delegate Custom|CheckScaleWeights) 1.0 true))
  (Variables|Default|SetTimer _returnvalue))

(fn ConstructionScript)

(fn MoveScale
  (bind _plates (Variables|Default|GetPlates))
  (bind _plates_2 (Variables|Default|GetPlates))
  (bind _plates_3 (Variables|Default|GetPlates))
  (bind _returnvalue (Transformation|GetWorldRotation _plates))
  (bind _returnvalue_2 (Transformation|GetWorldRotation _plates_2))
  (bind _returnvalue_3 (Transformation|GetWorldRotation _plates_3))
  (if (== (Variables|Default|GetLeftSideCurrentWeight) (Variables|Default|GetRightSideCurrentWeight))
    ;[1 1 1] Equal
    (Transformation|SetWorldLocationAndRotation _plates_2 (Transformation|GetWorldLocation _plates_2) (Math|Rotator|MakeRotator (.roll _returnvalue_2) 0.0 (.yaw _returnvalue_2)) false false)
    (elif (not (> (Variables|Default|GetLeftSideCurrentWeight) (Variables|Default|GetRightSideCurrentWeight)))
      ;[1 1 1] Left heavier
      (Transformation|SetWorldLocationAndRotation _plates (Transformation|GetWorldLocation _plates) (Math|Rotator|MakeRotator (.roll _returnvalue) (Variables|Default|GetLeftRotation) (.yaw _returnvalue)) false false)
      (else
        ;[1 1 1] Right heavier
        (Transformation|SetWorldLocationAndRotation _plates_3 (Transformation|GetWorldLocation _plates_3) (Math|Rotator|MakeRotator (.roll _returnvalue_3) (Variables|Default|GetRightRotation) (.yaw _returnvalue_3)) false false)))))

(fn OnPuzzleComplete
  (if (Utilities|Time|IsValidTimerHandle (Variables|Default|GetTimer))
    (Utilities|Time|ClearandInvalidateTimerbyHandle (Variables|Default|GetTimer))))