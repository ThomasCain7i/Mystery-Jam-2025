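; Child variant of the weight-checking plate in the Gluttony puzzle that totals the weight of items around it when play begins.
; After the parent BeginPlay, a multi sphere trace at the plate's location finds nearby actors within the check radius, with persistent debug drawing.
; Hits carrying a BPC_ItemHasWeight component add their weight to TotalWeight.
; The interact interface event is an empty stub with no parent call.
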(event EventBeginPlay
  (bind _self self)
  (bind _returnvalue (Transformation|GetActorLocation _self))
  (|CallParentFunction)
  (bind (_outhits _returnvalue_2) (Collision|MultiSphereTraceForObjects _returnvalue _returnvalue (Variables|Default|GetWeightCheckRadius) (Variables|Default|GetObjectTypes) false (Utilities|Array|MakeArray _self) "Persistent"))
  (if _returnvalue_2
    (for _array_element _outhits
      (Utilities|IsValid (Actor|GetComponentbyClass (.HitActor (Collision|BreakHitResult _array_element)) "/Game/Mike/Puzzles/Gluttony/BPC_ItemHasWeight.BPC_ItemHasWeight_C")
        (:Is%20Valid
          (bind _weight (Default|GetItemWeight (Actor|GetComponentbyClass (.HitActor (Collision|BreakHitResult _array_element)) "/Game/Mike/Puzzles/Gluttony/BPC_ItemHasWeight.BPC_ItemHasWeight_C")))
          (Variables|Default|SetTotalWeight (+ _weight (Variables|Default|GetTotalWeight))))))))

(event EventInterfaceInteract)

(fn ConstructionScript
  (|CallParentFunction))