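; BP_FoodPlate is a puzzle plate for the Gluttony puzzle that totals the weight of food placed on it.
; CheckPlateWeight resets the total, runs a multi-sphere object trace at the plate and sums BPC_ItemHasWeight values from hit actors carrying the food tag.
; It returns that total when the trace hits.
; The collider's overlap event is empty, leaving its pass-check logic disconnected and GoalWeight unused.
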(event OnComponentBeginOverlap(Collider)
  (params (OverlappedComponent :type Primitive%20Component%20Object%20Reference) (OtherActor :type Actor%20Object%20Reference) (OtherComp :type Primitive%20Component%20Object%20Reference) (OtherBodyIndex :type Integer) (bFromSweep :type Boolean) (SweepResult :type Hit%20Result%20Structure%20%28by%20ref%29)))

(fn ConstructionScript)

(fn CheckPlateWeight
  (bind _self self)
  (bind _defaultsceneroot (Variables|Default|GetDefaultSceneRoot _self))
  (bind _returnvalue (Transformation|GetWorldLocation _defaultsceneroot))
  (CallFunction|ClearPlateWeight)
  (bind (_outhits _returnvalue_2) (Collision|MultiSphereTraceForObjects _returnvalue (+ _returnvalue "1.000000,1.000000,1.000000") (Variables|Default|GetSphereTrace) (Variables|Default|GetObject%20Types) false (Utilities|Array|MakeArray self) "ForDuration"))
  (if _returnvalue_2
    (for _array_element _outhits
      (if (Actor|ActorHasTag (.HitActor (Collision|BreakHitResult _array_element)) (Variables|Default|GetFoodTag))
        (bind _weight (Default|GetItemWeight (Actor|GetComponentbyClass (.HitActor (Collision|BreakHitResult _array_element)) "/Game/Mike/Puzzles/Gluttony/BPC_ItemHasWeight.BPC_ItemHasWeight_C")))
        (Variables|Default|SetCurrentTotalWeight (+ _weight (Variables|Default|GetCurrentTotalWeight)))))
    (return (Variables|Default|GetCurrentTotalWeight))))

(fn ClearPlateWeight
  (Variables|Default|SetCurrentTotalWeight 0))