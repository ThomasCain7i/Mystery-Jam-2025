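; BP_GluttonyFoodPlate is a food plate for the Gluttony puzzle that totals the weight of items on or near it.
; On BeginPlay, a small sphere trace at its location gathers overlapping objects and adds the weight from each one's BPC_ItemHasWeight component to PlateTotalWeight.
; The tally runs only once, with persistent trace drawing and a debug print for hits lacking the component.
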(event EventBeginPlay
  (bind _self self)
  (bind _returnvalue (Transformation|GetActorLocation _self))
  (bind _outhits (Collision|MultiSphereTraceForObjects _returnvalue _returnvalue 2e+01 (Variables|Default|GetObject%20Types) false 0 "Persistent"))
  (for _array_element _outhits
    (Utilities|IsValid (Actor|GetComponentbyClass (.HitActor (Collision|BreakHitResult _array_element)) "/Game/Mike/Puzzles/Gluttony/BPC_ItemHasWeight.BPC_ItemHasWeight_C")
      (:Is%20Valid
        (bind _weight (Default|GetItemWeight (Actor|GetComponentbyClass (.HitActor (Collision|BreakHitResult _array_element)) "/Game/Mike/Puzzles/Gluttony/BPC_ItemHasWeight.BPC_ItemHasWeight_C")))
        (Variables|Default|SetPlateTotalWeight (+ _weight (Variables|Default|GetPlateTotalWeight))))
      (:Is%20Not%20Valid
        (Development|PrintString "Not valid " true true "(R=1.000000,G=0.177722,B=0.082038,A=1.000000)")))))

(fn ConstructionScript)