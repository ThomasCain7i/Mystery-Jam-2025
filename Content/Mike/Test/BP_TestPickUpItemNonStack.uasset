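; BP_TestPickUpItemNonStack is a test interactable pickup actor, named as a non-stacking item.
; On BeginPlay it passes its cube mesh to the BPCInteractWithItem component as item mesh data.
; Interface events toggle custom depth on the cube for focus and handle interaction, and an interface function returns its widget.
; Each interaction flips the point light's visibility and calls PickUpItem on the component in both toggle states.
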(event Custom|UseInteract
  (bind _bpc_interactwithitem (Variables|Default|GetBPC_InteractWithItem))
  (bind _pointlight (Variables|Default|GetPointLight))
  (bind _output_get (Variables|Default|SetInteractToggle (not (Variables|Default|GetInteractToggle))))
  (if _output_get
    (Rendering|SetVisibility _pointlight true false)
    (Default|PickUpItem _bpc_interactwithitem)
    (else
      (Rendering|SetVisibility _pointlight false false)
      (Default|PickUpItem _bpc_interactwithitem))))

(event EventBeginPlay
  (Default|SetUpItemMeshData (Variables|Default|GetBPC_InteractWithItem) (Variables|/Script/Engine.StaticMeshComponent|GetStaticMesh (Variables|Default|GetCube))))

(event EventInterfaceToggleFocus
  (params (Focus :type Boolean))
  (Rendering|SetRenderCustomDepth (Variables|Default|GetCube) Focus))

(event EventInterfaceInteract
  (CallFunction|UseInteract))

(fn ConstructionScript)

(fn InterfaceGetInteractionWidgetRef
  (return (Variables|Default|GetWidget)))