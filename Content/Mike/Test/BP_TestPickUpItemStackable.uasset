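; Test actor for a stackable pickup item that the player can focus and interact with through an interaction interface.
; Focus toggles custom depth rendering on the cube, and the interface also returns a reference to the interaction widget.
; Each interaction flips a toggle that shows or hides the point light, and both branches call PickUpItem on the pickup component.
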(event Custom|UseInteract
  (bind _pointlight (Variables|Default|GetPointLight))
  (bind _output_get (Variables|Default|SetInteractToggle (not (Variables|Default|GetInteractToggle))))
  (if _output_get
    (Rendering|SetVisibility _pointlight true false)
    (Default|PickUpItem (Variables|Default|GetBPC_PickUpItem))
    (else
      (Rendering|SetVisibility _pointlight false false)
      (Default|PickUpItem (Variables|Default|GetBPC_PickUpItem)))))

(event EventBeginPlay)

(event Collision|EventActorBeginOverlap
  (params (OtherActor :type Actor%20Object%20Reference)))

(event EventTick
  (params (DeltaSeconds :type Float%20%28single-precision%29)))

(event EventInterfaceToggleFocus
  (params (Focus :type Boolean))
  (Rendering|SetRenderCustomDepth (Variables|Default|GetCube) Focus))

(event EventInterfaceInteract
  (CallFunction|UseInteract))

(fn ConstructionScript)

(fn InterfaceGetInteractionWidgetRef
  (return (Variables|Default|GetWidget)))