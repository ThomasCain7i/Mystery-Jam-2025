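; Inspection actor that shows a picked item's mesh via a SceneCapture2D with a name and description widget.
; Inspect swaps input from the character to itself; mouse drag or move input rotates the item, wheel or Z/X zooms by clamped capture FOV, and right-click resets.
; Interact restores character input, removes the widget and destroys the actor.
; Setter functions adjust the item's starting rotation, scale, offset and FOV.
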(event Input|EnhancedActionEvents|EnhancedInputActionIA_Interact
  (params (ActionValue :type Boolean) (ElapsedSeconds :type Float%20%28double-precision%29) (TriggeredSeconds :type Float%20%28double-precision%29) (InputAction :type Input%20Action%20Object%20Reference :default "/Game/FirstPerson/Input/Actions/IA_Interact.IA_Interact"))
  (bind _returnvalue (Game|GetPlayerController 0))
  ;[1 1 1] Close inspect item screen and enable input for character
  (:Started
    (Input|DisableInput _returnvalue)
    (Input|EnableInput (Variables|Default|GetCharacter) _returnvalue)
    (Utilities|IsValid (Variables|Default|GetItemInspectWidgetRef)
      (:Is%20Valid
        ;;[1 0.6426 0.3986] Remove Widget from screen by setting to none
        (Widget|RemovefromParent (Variables|Default|GetItemInspectWidgetRef))
        (Variables|Default|SetItemInspectWidgetRef 0)
        (Actor|DestroyActor)))))

(event Input|EnhancedActionEvents|EnhancedInputActionIA_Move
  (params (ActionValue :type Vector%202D%20Structure) (ElapsedSeconds :type Float%20%28double-precision%29) (TriggeredSeconds :type Float%20%28double-precision%29) (InputAction :type Input%20Action%20Object%20Reference :default "/Game/FirstPerson/Input/Actions/IA_Move.IA_Move"))
  ;[0.01729 0.0183 0.02604] Controlling inspect item
  ;;[1 0.7146 0.1739] Interact movement with WASD
  (if (or (!= (.x ActionValue) 0.0) (!= (.y ActionValue) 0.0))
    (Utilities|FlowControl|Sequence
      (:then_0
        (Transformation|SetWorldRotation (Variables|Default|GetItem) (Math|Rotator|CombineRotators (Transformation|GetWorldRotation (Variables|Default|GetItem)) (Math|Rotator|MakeRotator 0.0 0.0 (* (.x ActionValue) (Variables|Default|GetRotateSpeed)))) false false))
      (:then_1
        (Transformation|SetWorldRotation (Variables|Default|GetItem) (Math|Rotator|CombineRotators (Transformation|GetWorldRotation (Variables|Default|GetItem)) (Math|Rotator|MakeRotator 0.0 (* (.y ActionValue) (Variables|Default|GetRotateSpeed)) 0.0)) false false)))))

(event EventInspect
  (params (Character :type BP%20First%20Person%20Character%20Object%20Reference) (InspectedItemMesh :type Static%20Mesh%20Object%20Reference) (ItemName :type String) (ItemDescription :type String))
  (bind _returnvalue (Game|GetPlayerController 0))
  ;[1 1 1] Create inspect HUD widget and enable input for Inspect
  (Development|PrintString "Inpspect")
  (Variables|Default|SetCharacter Character)
  (Utilities|IsValid InspectedItemMesh
    (:Is%20Valid
      (Components|StaticMesh|SetStaticMesh (Variables|Default|GetItem) InspectedItemMesh)
      (bind _returnvalue_2 (UserInterface|CreateWidget "/Game/Mike/Inspect/WB_ItemInspect.WB_ItemInspect_C" 0 (Utilities|Text|ToText(String) ItemName) (Utilities|Text|ToText(String) ItemDescription)))
      (bind _output_get (Variables|Default|SetItemInspectWidgetRef _returnvalue_2))
      (UserInterface|Viewport|AddtoViewport _output_get 0)
      (Input|DisableInput (Variables|Default|GetCharacter) _returnvalue)
      (Input|EnableInput _returnvalue))))

(event Input|MouseEvents|MouseX
  (params (AxisValue :type Float%20%28single-precision%29))
  (bind _item (Variables|Default|GetItem))
  ;[0.01729 0.0183 0.02604] Controlling inspect item
  ;;[0.1986 0.8942 1] Inspect horizontal mouse controls
  (if (Variables|Default|GetbCanRotate)
    (Transformation|SetWorldRotation _item (Math|Rotator|CombineRotators (Transformation|GetWorldRotation _item) (Math|Rotator|MakeRotator 0.0 0.0 (* AxisValue (Variables|Default|GetRotateSpeed)))) false false)))

(event Input|MouseEvents|MouseY
  (params (AxisValue :type Float%20%28single-precision%29))
  (bind _item (Variables|Default|GetItem))
  ;[0.01729 0.0183 0.02604] Controlling inspect item
  ;;[0.1986 0.8942 1] Inspect vertical mouse controls
  (if (Variables|Default|GetbCanRotate)
    (Transformation|SetWorldRotation _item (Math|Rotator|CombineRotators (Transformation|GetWorldRotation _item) (Math|Rotator|MakeRotator 0.0 (* AxisValue (Variables|Default|GetRotateSpeed)) 0.0)) false false)))

(event Input|MouseEvents|LeftMouseButton
  (params (Key :type Key%20Structure :default "None"))
  ;[0.01729 0.0183 0.02604] Controlling inspect item
  ;;[0.1986 0.8942 1] Check is holding mouse down
  (:Pressed
    (Variables|Default|SetbCanRotate true))
  (:Released
    (Variables|Default|SetbCanRotate false)))

(event Input|MouseEvents|RightMouseButton
  (params (Key :type Key%20Structure :default "None"))
  ;[0.01729 0.0183 0.02604] Controlling inspect item
  ;;[0.1986 0.8942 1] Reset Inspected Item Transform
  (:Pressed
    (Transformation|SetWorldRotation (Variables|Default|GetItem) (Variables|Default|GetItemRotation) false false)
    (Variables|/Script/Engine.SceneCaptureComponent2D|SetFOVAngle (Variables|Default|GetSceneCaptureComponent2D) (Variables|Default|GetStartInspectFOV))))

(event Input|MouseEvents|MouseWheelUp
  (params (Key :type Key%20Structure :default "None"))
  (bind _scenecapturecomponent2d (Variables|Default|GetSceneCaptureComponent2D))
  ;[0.01729 0.0183 0.02604] Controlling inspect item
  ;;[0.1986 0.8942 1] Zoom In and Out Mouse
  (:Pressed
    (Variables|/Script/Engine.SceneCaptureComponent2D|SetFOVAngle _scenecapturecomponent2d (Math|Float|Clamp(Float) (- (Variables|/Script/Engine.SceneCaptureComponent2D|GetFOVAngle _scenecapturecomponent2d) 1.0) (Variables|Default|GetMinFOV) (Variables|Default|GetMaxFOV)))))

(event Input|MouseEvents|MouseWheelDown
  (params (Key :type Key%20Structure :default "None"))
  (bind _scenecapturecomponent2d (Variables|Default|GetSceneCaptureComponent2D))
  ;[0.01729 0.0183 0.02604] Controlling inspect item
  ;;[0.1986 0.8942 1] Zoom In and Out Mouse
  (:Pressed
    (Variables|/Script/Engine.SceneCaptureComponent2D|SetFOVAngle _scenecapturecomponent2d (Math|Float|Clamp(Float) (+ (Variables|/Script/Engine.SceneCaptureComponent2D|GetFOVAngle _scenecapturecomponent2d) 1.0) (Variables|Default|GetMinFOV) (Variables|Default|GetMaxFOV)))))

(event Input|KeyboardEvents|Z
  (params (Key :type Key%20Structure :default "None"))
  (bind _scenecapturecomponent2d (Variables|Default|GetSceneCaptureComponent2D))
  ;[0.01729 0.0183 0.02604] Controlling inspect item
  ;;[1 0.7146 0.1739] Zoom In and Out Keyboard
  (:Pressed
    (Variables|/Script/Engine.SceneCaptureComponent2D|SetFOVAngle _scenecapturecomponent2d (Math|Float|Clamp(Float) (- (Variables|/Script/Engine.SceneCaptureComponent2D|GetFOVAngle _scenecapturecomponent2d) 1.0) (Variables|Default|GetMinFOV) (Variables|Default|GetMaxFOV)))))

(event Input|KeyboardEvents|X
  (params (Key :type Key%20Structure :default "None"))
  (bind _scenecapturecomponent2d (Variables|Default|GetSceneCaptureComponent2D))
  ;[0.01729 0.0183 0.02604] Controlling inspect item
  ;;[1 0.7146 0.1739] Zoom In and Out Keyboard
  (:Pressed
    (Variables|/Script/Engine.SceneCaptureComponent2D|SetFOVAngle _scenecapturecomponent2d (Math|Float|Clamp(Float) (+ (Variables|/Script/Engine.SceneCaptureComponent2D|GetFOVAngle _scenecapturecomponent2d) 1.0) (Variables|Default|GetMinFOV) (Variables|Default|GetMaxFOV)))))

(fn ConstructionScript)

(fn SetInspectRotation
  (params (ItemRotation :type Rotator))
  (bind _item (Variables|Default|GetItem))
  (bind _returnvalue (Transformation|GetWorldTransform _item))
  (bind _output_get (Variables|Default|SetItemRotation ItemRotation))
  (Transformation|SetWorldTransform _item (Math|Transform|MakeTransform (.location _returnvalue) _output_get (.scale _returnvalue)) false false))

(fn SetInspectScale
  (params (InspectScale :type Vector))
  (bind _item (Variables|Default|GetItem))
  (bind _returnvalue (Transformation|GetWorldTransform _item))
  (Transformation|SetWorldTransform _item (Math|Transform|MakeTransform (.location _returnvalue) (.rotation _returnvalue) InspectScale) false false))

(fn SetInspectOffsetLocation
  (params (OffsetLocation :type Vector))
  (bind _item (Variables|Default|GetItem))
  (bind _returnvalue (Transformation|GetWorldTransform _item))
  (Transformation|SetWorldTransform _item (Math|Transform|MakeTransform (+ OffsetLocation (.location _returnvalue)) (.rotation _returnvalue) (.scale _returnvalue)) false false))

(fn SetStartInspectFOV
  (params (NewFOV :type Float%20%28double-precision%29))
  (Variables|/Script/Engine.SceneCaptureComponent2D|SetFOVAngle (Variables|Default|GetSceneCaptureComponent2D) (Math|Float|Clamp(Float) (Variables|Default|GetStartInspectFOV) (Variables|Default|GetMinFOV) (Variables|Default|GetMaxFOV))))