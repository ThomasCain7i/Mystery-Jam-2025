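; BP_Inventory is an inventory Blueprint that stores items as an array of slot structs, each holding item data and a quantity.
; The AddItem event validates the item, then FindNextSlot picks the first slot with the same item if it is stackable, or requests a new slot.
; The AddItem function then appends a slot or increases the existing quantity with no stack limit, printing debug messages.
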(event Custom|Add%20Item
  (params (Item :type DA%20Item%20Object%20Reference) (Quantity :type Integer))
  (Utilities|IsValid Item
    (:Is%20Valid
      (bind (_bcreatenewslot _inventoryindex) (CallFunction|FindNextSlot Item))
      (CallFunction|AddItem Item Quantity _inventoryindex _bcreatenewslot))
    (:Is%20Not%20Valid
      (Development|PrintString "Item not valid" true true "(R=1.000000,G=0.000000,B=0.044383,A=1.000000)"))))

(fn ConstructionScript)

(fn FindNextSlot
  (params (Item :type DA%20Item%20Object%20Reference))
  (if (.bIsStackable (Utilities|Struct|BreakST_Item (Variables|/Game/Mike/Blueprints/Inventory/DA_Item.DA_Item_C|GetItemData Item)))
    (bind (_array_element _array_index) (Utilities|Array|ForEachLoopwithBreak (Variables|Default|GetInventorySlots))
      (:LoopBody
        (if (== (.ItemData (Utilities|Struct|BreakST_InventorySlot _array_element)) Item)
          (return false _array_index)))
      (:Completed
        (return true 0)))
    (else
      (return true 0))))

(fn AddItem
  (params (Item%20Data :type DA%20Item%20Object%20Reference) (Quantity :type Integer) (InventoryIndex :type Integer) (bCreateNewSlot :type Boolean))
  (if bCreateNewSlot
    ;[0.1712 1 0.3023] Add item to new slot
    (Utilities|Array|Add (Variables|Default|GetInventorySlots) (Utilities|Struct|MakeST_InventorySlot Item%20Data Quantity))
    (Variables|Default|SetInventorySlots (Variables|Default|GetInventorySlots))
    (Development|PrintString "Item added to a new slot " true true "(R=0.147600,G=1.000000,B=0.134544,A=1.000000)" 4.0)
    (else
      ;[0.2552 0.2071 1] Add Item to existing slot
      (Utilities|Array|SetArrayElem (Variables|Default|GetInventorySlots) InventoryIndex (Utilities|Struct|MakeST_InventorySlot Item%20Data (+ (.Quantity (Utilities|Struct|BreakST_InventorySlot (Utilities|Array|Get(acopy) (Variables|Default|GetInventorySlots) InventoryIndex))) Quantity)))
      (Variables|Default|SetInventorySlots (Variables|Default|GetInventorySlots))
      (Development|PrintString "Item added to existing slot"))))