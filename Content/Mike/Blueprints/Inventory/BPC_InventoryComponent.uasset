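; Inventory component that holds a fixed-size item array, creates its WB_Inventory widget on BeginPlay and opens it in UI-only mode on IA_Inventory.
; TryAddToInventory walks the slots, stacking matching stackable items below MaxAmount or inserting into a zero-quantity slot.
; A successful add refreshes the widget and destroys the pickup's owning actor.
; The pickup event is empty, and its binding and TryAddToInventory call are unwired in the EventGraph.
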(event Custom|TryPickUpNewItem_Event
  (params (PickUpItem :type BPC%20Pick%20Up%20Item%20Object%20Reference))
  ;[1 1 1] Try and pick up a new item
)

(event Input|EnhancedActionEvents|EnhancedInputActionIA_Inventory
  (params (ActionValue :type Boolean) (ElapsedSeconds :type Float%20%28double-precision%29) (TriggeredSeconds :type Float%20%28double-precision%29) (InputAction :type Input%20Action%20Object%20Reference :default "/Game/FirstPerson/Input/Actions/IA_Inventory.IA_Inventory"))
  (bind _returnvalue (Game|GetPlayerController 0))
  (bind _inventoryref (Variables|Default|GetInventoryRef))
  (bind _inventoryref_2 (Variables|Default|GetInventoryRef))
  ;[1 1 1] Opening Inventory
  (Development|PrintString "Opened inventory")
  (if (not (UserInterface|Viewport|IsinViewport _inventoryref))
    (UserInterface|Viewport|AddtoViewport _inventoryref 0)
    (Variables|/Script/Engine.PlayerController|SetbShowMouseCursor _returnvalue true)
    (Input|SetInputModeUIOnly _returnvalue _inventoryref_2 "DoNotLock" false)
    (Variables|/Script/UMG.UserWidget|SetbIsFocusable _inventoryref_2 true)))

(event EventBeginPlay
  ;[1 1 1] On Start
  (bind _returnvalue (UserInterface|CreateWidget "/Game/Mike/Hud/Inventory/WB_Inventory.WB_Inventory_C"))
  (Variables|Default|SetInventoryRef _returnvalue)
  (Utilities|Array|Resize (Variables|Default|GetItems) (Variables|Default|GetInventorySize))
  (Default|RefreshInventory (Variables|Default|GetInventoryRef) self)
  (Development|PrintString "Hello"))

(fn TryAddtoInventory
  (params (Item :type BPC%20Pick%20Up%20Item%20Object%20Reference))
  (bind _items (Variables|Default|GetItems))
  (LocalVariables|SetPickUpItemData Item)
  (for (_array_element _array_index) (Variables|Default|GetItems)
    (Utilities|IsValid (LocalVariables|GetPickUpItemData)
      (:Is%20Valid
        (Variables|Default|SetCurrentIndex _array_index)
        (bind (_bisstackable _newquantity) (CallFunction|CheckIsStackable _array_element (Variables|/Game/Mike/Blueprints/Inventory/BPC_PickUpItem.BPC_PickUpItem_C|GetItem (LocalVariables|GetPickUpItemData))))
        (if _bisstackable
          (Development|PrintString "New Item added to current stack" true true "(R=0.084933,G=1.000000,B=0.056737,A=1.000000)" 5.0)
          ;[1 1 1] Stack pick up item
          (bind _output_get (Variables|Default|SetUpdatedQuantity _newquantity))
          (Utilities|Array|SetArrayElem (Variables|Default|GetItems) (Variables|Default|GetCurrentIndex) (Utilities|Struct|MakeST_Item (.Name (Utilities|Struct|BreakST_Item (Variables|/Game/Mike/Blueprints/Inventory/BPC_PickUpItem.BPC_PickUpItem_C|GetItem (LocalVariables|GetPickUpItemData)))) (.Description (Utilities|Struct|BreakST_Item (Variables|/Game/Mike/Blueprints/Inventory/BPC_PickUpItem.BPC_PickUpItem_C|GetItem (LocalVariables|GetPickUpItemData)))) (.Icon (Utilities|Struct|BreakST_Item (Variables|/Game/Mike/Blueprints/Inventory/BPC_PickUpItem.BPC_PickUpItem_C|GetItem (LocalVariables|GetPickUpItemData)))) (.ItemType (Utilities|Struct|BreakST_Item (Variables|/Game/Mike/Blueprints/Inventory/BPC_PickUpItem.BPC_PickUpItem_C|GetItem (LocalVariables|GetPickUpItemData)))) (.bIsStackable (Utilities|Struct|BreakST_Item (Variables|/Game/Mike/Blueprints/Inventory/BPC_PickUpItem.BPC_PickUpItem_C|GetItem (LocalVariables|GetPickUpItemData)))) (.bCanPickUp (Utilities|Struct|BreakST_Item (Variables|/Game/Mike/Blueprints/Inventory/BPC_PickUpItem.BPC_PickUpItem_C|GetItem (LocalVariables|GetPickUpItemData)))) _output_get (.ItemMesh (Utilities|Struct|BreakST_Item (Variables|/Game/Mike/Blueprints/Inventory/BPC_PickUpItem.BPC_PickUpItem_C|GetItem (LocalVariables|GetPickUpItemData))))))
          (Default|RefreshInventory (Variables|Default|GetInventoryRef) self :!label _label)
          (Actor|DestroyActor (Components|GetOwner (LocalVariables|GetPickUpItemData)))
          (return)
          (else
            (bind _bisinventoryfull (CallFunction|CheckifInventoryFull _newquantity))
            (if _bisinventoryfull
              (Development|PrintString (Utilities|String|Append (.Name (Utilities|Struct|BreakST_Item (Variables|/Game/Mike/Blueprints/Inventory/BPC_PickUpItem.BPC_PickUpItem_C|GetItem (LocalVariables|GetPickUpItemData)))) " can't be picked up, Inventory is full!") true true "(R=1.000000,G=0.264888,B=0.029167,A=1.000000)" 5.0)
              (else
                ;[1 1 1] Insert new Item to inventory
                (Utilities|Array|Insert _items (Variables|/Game/Mike/Blueprints/Inventory/BPC_PickUpItem.BPC_PickUpItem_C|GetItem (LocalVariables|GetPickUpItemData)) (Variables|Default|GetCurrentIndex))
                (Utilities|Array|RemoveIndex _items (- (Variables|Default|GetInventorySize) (Variables|Default|GetCurrentIndex)))
                (goto _label))))))
      (:Is%20Not%20Valid
        (Development|PrintString "Actor Not Valid Pick Up!!" true true "(R=1.000000,G=0.204888,B=0.125190,A=1.000000)" 5.0)))))

(fn CheckIsStackable
  (params (ItemInventory :type ST%20Item%20Structure) (ItemPickUp :type ST%20Item%20Structure))
  (bind (_name _description _icon _itemtype _bisstackable _bcanpickup _itemamount) (Utilities|Struct|BreakST_Item ItemInventory))
  (bind (_name_2 _description_2 _icon_2 _itemtype_2 _bisstackable_2 _bcanpickup_2 _itemamount_2) (Utilities|Struct|BreakST_Item ItemPickUp))
  (bind _returnvalue (+ _itemamount _itemamount_2))
  ;[1 0.03137 0] If not the same item return
  (if (Utilities|Enum|NotEqual(Enum) _name _name_2)
    _
    (else
      ;[1 0.03137 0] If not stackable return
      (if (not (Math|Boolean|ANDBoolean _bisstackable _bisstackable_2 _bcanpickup_2))
        _
        (elif (>= _returnvalue (Variables|Default|GetMaxAmount))
          _
          (else
            (return true _returnvalue))))))
  (return false _itemamount))

(fn CheckifInventoryFull
  (params (CurrentSlotQuantity :type Integer))
  (if (== CurrentSlotQuantity 0)
    ;[1 1 1] Check if there is any item in the current inventory index by checking its amount (if 0 then there is no item)
    (return false)
    (else
      (return true))))