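; Inventory component that stores an item array and opens the inventory screen on input.
; On BeginPlay it creates the WB_Inventory widget, sizes the item array to the maximum inventory size and passes itself to the widget to refresh the display.
; The IA_Inventory action adds the widget to the viewport if absent, shows the cursor and switches player 0 to UI-only input.
; This graph only opens the screen and has no closing logic.
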(event Input|EnhancedActionEvents|EnhancedInputActionIA_Inventory
  (params (ActionValue :type Vector%202D%20Structure) (ElapsedSeconds :type Float%20%28double-precision%29) (TriggeredSeconds :type Float%20%28double-precision%29) (InputAction :type Input%20Action%20Object%20Reference :default "/Game/FirstPerson/Input/Actions/IA_Inventory.IA_Inventory"))
  (bind _returnvalue (Game|GetPlayerController 0))
  (bind _inventoryref (Variables|Default|GetInventoryRef))
  (bind _inventoryref_2 (Variables|Default|GetInventoryRef))
  ;[1 1 1] Open Inventory
  (if (not (UserInterface|Viewport|IsinViewport _inventoryref))
    (UserInterface|Viewport|AddtoViewport _inventoryref 0)
    (Variables|/Script/Engine.PlayerController|SetbShowMouseCursor _returnvalue true)
    (Input|SetInputModeUIOnly _returnvalue _inventoryref_2 "DoNotLock" false)
    (Variables|/Script/UMG.UserWidget|SetbIsFocusable _inventoryref_2 true)))

(event EventBeginPlay
  (bind _returnvalue (UserInterface|CreateWidget "/Game/Mike/Inventory/HUD/WB_Inventory.WB_Inventory_C"))
  (bind _output_get (Variables|Default|SetInventoryRef _returnvalue))
  (Utilities|Array|Resize (Variables|Default|GetInventoryItems) (Variables|Default|GetMaxInventorySize))
  (Default|RefreshInventory _output_get self))