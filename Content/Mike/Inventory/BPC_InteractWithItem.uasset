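; Item component that holds an item's data struct and handles player interaction for inspecting it and picking it up.
; PickUpItem casts to the first-person character, then runs inspection and an inventory add attempt in sequence, each gated by its own item flag.
; Inspection spawns a BP_InspectItem far outside the level, passing it mesh, text, transform tweaks and an optional start FOV override.
; A separate event can set the item mesh at runtime.
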(event Custom|SetUpItemMeshData
  (params (PickUpItemMesh :type Static%20Mesh%20Object%20Reference))
  ;[1 1 1] Set the items mesh data through blueprints instead of in data component (not needed)
  ;;[0.9927 0 0.04745] Need to manually re-connect if you change Struct for item REDO
  (bind _output_get (Variables|Data|SetItemData (Utilities|Struct|MakeST_Item PickUpItemMesh (.Name (Utilities|Struct|BreakST_Item (Variables|Data|GetItemData))) (.Description (Utilities|Struct|BreakST_Item (Variables|Data|GetItemData))) (.Icon (Utilities|Struct|BreakST_Item (Variables|Data|GetItemData))) (.bCanInspect (Utilities|Struct|BreakST_Item (Variables|Data|GetItemData))) (.bCanPickUp (Utilities|Struct|BreakST_Item (Variables|Data|GetItemData))) (.bIsStackable (Utilities|Struct|BreakST_Item (Variables|Data|GetItemData))) (.bIsUsable (Utilities|Struct|BreakST_Item (Variables|Data|GetItemData))) (.bCanDelete (Utilities|Struct|BreakST_Item (Variables|Data|GetItemData))) (.ItemQuantity (Utilities|Struct|BreakST_Item (Variables|Data|GetItemData))) (.ItemInspectionRotation (Utilities|Struct|BreakST_Item (Variables|Data|GetItemData))) (.ItemInspectionScale (Utilities|Struct|BreakST_Item (Variables|Data|GetItemData))) (.ItemInspectionOffsetLocation (Utilities|Struct|BreakST_Item (Variables|Data|GetItemData)))))))

(event Custom|PickUpItem
  (bind _itemdata (Variables|Data|GetItemData))
  (bind (_itemmesh _name _description _icon _bcaninspect _bcanpickup) (Utilities|Struct|BreakST_Item _itemdata))
  ;[1 1 1] Try Pick Up Item
  (bind _asbp_first_person_character (Utilities|Casting|CastToBP_FirstPersonCharacter (Game|GetPlayerCharacter 0)))
  (Variables|PickUp|SetFirstPersonCharacterRef _asbp_first_person_character)
  (Utilities|FlowControl|Sequence
    (:then_0
      ;[1 1 1] Inspect Item
      (if _bcaninspect
        (CallFunction|InspectItem (Variables|PickUp|GetFirstPersonCharacterRef))))
    (:then_1
      ;[1 1 1] Pick Up item
      (if _bcanpickup
        (Default|TryAddtoInventory (Variables|/Game/FirstPerson/Blueprints/BP_FirstPersonCharacter.BP_FirstPersonCharacter_C|GetBPC_InventoryComponent (Variables|PickUp|GetFirstPersonCharacterRef)) self)))))

(fn InspectItem
  (params (FirstPersonPlayerRef :type BP%20First%20Person%20Character%20Object%20Reference))
  (bind _itemdata (Variables|Data|GetItemData))
  (bind _itemdata_2 (Variables|Data|GetItemData))
  (bind (_itemmesh _name _description _icon _bcaninspect _bcanpickup _bisstackable _bisusable _bcandelete _itemquantity _iteminspectionrotation _iteminspectionscale _iteminspectionoffsetlocation) (Utilities|Struct|BreakST_Item _itemdata))
  (bind (_itemmesh_2 _name_2 _description_2) (Utilities|Struct|BreakST_Item _itemdata_2))
  (bind _returnvalue (Game|SpawnActorfromClass "/Game/Mike/Inspect/BP_InspectItem.BP_InspectItem_C" (Math|Transform|MakeTransform "100000000.000000,0.000000,0.000000") "Undefined" "MultiplyWithRoot" 0 0))
  (Default|SetInspectOffsetLocation _returnvalue _iteminspectionoffsetlocation)
  (Default|SetInspectScale _returnvalue _iteminspectionscale)
  (Default|SetInspectRotation _returnvalue _iteminspectionrotation)
  (if (not (Variables|Inspect|GetbOverrideInspectFOV))
    _
    (else
      ;[1 1 1] Override start FOV
      (Default|SetStartInspectFOV _returnvalue (Variables|Inspect|GetItemInspectStartFOV))))
  (Class|BIInspectInterface|InspectItem(Message) _returnvalue FirstPersonPlayerRef _itemmesh_2 _name_2 _description_2))

(fn InterfaceGetInteractionWidgetRef
  (return 0))