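; Actor component that lets a player pick up, carry and drop physics objects through a physics handle and camera supplied by the caller.
; Grabbing line-traces along the camera's forward vector and holds the hit component at its own location.
; An update event, driven externally, moves the handle target to the hold distance in front of the camera.
; While holding, the mouse wheel adjusts that distance within clamped limits, and release restores the default.
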(event Custom|GrabActor
  (params (PhysicsHandle :type Physics%20Handle%20Component%20Object%20Reference) (Camera :type Camera%20Component%20Object%20Reference))
  (bind _returnvalue (Transformation|GetWorldLocation Camera))
  ;[1 1 1] Grab other actors
  (bind (_outhit _returnvalue_2) (Collision|LineTraceForObjects _returnvalue (+ _returnvalue (* (Math|Vector|GetForwardVector Camera) (Variables|Default|GetGrabDistance))) (Variables|Default|GetObject%20Types) false 0 "None"))
  (if _returnvalue_2
    (Physics|Components|PhysicsHandle|GrabComponentatLocationwithRotation PhysicsHandle (.HitComponent (Collision|BreakHitResult _outhit)) "None" (Transformation|GetWorldLocation (.HitComponent (Collision|BreakHitResult _outhit))) "0, 0, 0")
    (Variables|Default|SetbIsGrabbing true)))

(event Custom|ReleaseActor
  (params (PhysicsHandle :type Physics%20Handle%20Component%20Object%20Reference))
  ;[1 1 1] Release the currently grabed item
  (if (Variables|Default|GetbIsGrabbing)
    (Physics|Components|PhysicsHandle|ReleaseComponent PhysicsHandle)
    (CallFunction|ResetHoldDistance)
    (Variables|Default|SetbIsGrabbing false)))

(event Custom|UpdatePickedUpActorLocation
  (params (PhysicsHandle :type Physics%20Handle%20Component%20Object%20Reference) (Camera :type Camera%20Component%20Object%20Reference))
  ;[1 1 1] Update grabbed items location
  (if (Variables|Default|GetbIsGrabbing)
    (Physics|Components|PhysicsHandle|SetTargetLocation PhysicsHandle (+ (Transformation|GetWorldLocation Camera) (* (Math|Vector|GetForwardVector Camera) (Variables|Default|GetHoldDistance))))))

(event Custom|ResetHoldDistance
  (Variables|Default|SetHoldDistance (Variables|Default|GetDefaultHoldDistance)))

(event EventBeginPlay
  (Variables|Default|SetDefaultHoldDistance (Variables|Default|GetHoldDistance)))

(event Input|MouseEvents|MouseWheelUp
  (params (Key :type Key%20Structure :default "None"))
  (:Pressed
    (if (Variables|Default|GetbIsGrabbing)
      (Variables|Default|SetHoldDistance (Math|Float|Clamp(Float) (+ (Variables|Default|GetHoldDistance) (Variables|Default|GetScrollSpeed)) 5e+01 3e+02)))))

(event Input|MouseEvents|MouseWheelDown
  (params (Key :type Key%20Structure :default "None"))
  (:Pressed
    (if (Variables|Default|GetbIsGrabbing)
      (Variables|Default|SetHoldDistance (Math|Float|Clamp(Float) (- (Variables|Default|GetHoldDistance) (Variables|Default|GetScrollSpeed)) 5e+01 3e+02)))))