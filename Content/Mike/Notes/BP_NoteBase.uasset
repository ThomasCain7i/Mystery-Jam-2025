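; BP_NoteBase is an interactable note actor that shows its text on screen when the player interacts with it.
; A GetPlayer overlap component caches the first-person character reference for later use.
; Reading creates a WB_ReadNote widget from NoteText, plays a pickup sound and moves input from the character to the note.
; IA_Interact then closes the note, removing the widget and returning input to the character.
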(event OnComponentBeginOverlap(GetPlayer)
  (params (OverlappedComponent :type Primitive%20Component%20Object%20Reference) (OtherActor :type Actor%20Object%20Reference) (OtherComp :type Primitive%20Component%20Object%20Reference) (OtherBodyIndex :type Integer) (bFromSweep :type Boolean) (SweepResult :type Hit%20Result%20Structure%20%28by%20ref%29))
  (bind _asbp_first_person_character (Utilities|Casting|CastToBP_FirstPersonCharacter OtherActor))
  (Variables|Default|SetAs%20BP%20First%20Person%20Character _asbp_first_person_character)
  (Development|PrintString "Set"))

(event Custom|ReadNote
  (bind _returnvalue (Game|GetPlayerController 0))
  (Development|PrintString "Reading note")
  (Variables|Default|SetbIsReading true)
  (bind _returnvalue_2 (UserInterface|CreateWidget "/Game/Mike/Inventory/HUD/WB_ReadNote.WB_ReadNote_C" 0 (Variables|Default|GetNoteText)))
  (bind _output_get (Variables|Default|SetReadNoteWidget _returnvalue_2))
  (UserInterface|Viewport|AddtoViewport _output_get 0)
  (Input|DisableInput (Variables|Default|GetAs%20BP%20First%20Person%20Character) _returnvalue)
  (Input|EnableInput _returnvalue)
  (Audio|PlaySound2D "/Game/Sounds/Player/PickUp/SC_PickUp.SC_PickUp" 1.0 1.0 0.0 0 0))

(event Custom|CloseNote
  (bind _returnvalue (Game|GetPlayerController 0))
  (Variables|Default|SetbIsReading false)
  (Input|DisableInput _returnvalue)
  (Input|EnableInput (Variables|Default|GetAs%20BP%20First%20Person%20Character) _returnvalue)
  (Utilities|IsValid (Variables|Default|GetReadNoteWidget)
    (:Is%20Valid
      ;[1 0.6426 0.3986] Remove Widget from screen by setting to none
      (Widget|RemovefromParent (Variables|Default|GetReadNoteWidget))
      (Variables|Default|SetReadNoteWidget 0))))

(event Input|EnhancedActionEvents|EnhancedInputActionIA_Interact
  (params (ActionValue :type Boolean) (ElapsedSeconds :type Float%20%28double-precision%29) (TriggeredSeconds :type Float%20%28double-precision%29) (InputAction :type Input%20Action%20Object%20Reference :default "/Game/FirstPerson/Input/Actions/IA_Interact.IA_Interact"))
  (:Started
    (if (Variables|Default|GetbIsReading)
      (CallFunction|CloseNote))))

(event EventBeginPlay)

(event Collision|EventActorBeginOverlap
  (params (OtherActor :type Actor%20Object%20Reference)))

(event EventTick
  (params (DeltaSeconds :type Float%20%28single-precision%29)))

(event EventInterfaceInteract
  (CallFunction|ReadNote))

(fn ConstructionScript)