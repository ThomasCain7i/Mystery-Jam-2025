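; Interaction component that line-traces from the player camera each tick to find and focus BP_InteractionArea box or custom-shape actors.
; Input on a focused area either interacts instantly or runs a looping timer that fills the area's WB_Interaction progress until its hold duration completes.
; Completion sends an interface interact message to the area's parent actor, with a test print for BP_TestBox.
; Releasing input or losing focus stops the hold.
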(event Custom|TryToInteract
  (params (Input :type Boolean))
  (if Input
    (if (Variables|Default|GetIsTracingInteractionArea)
      (bind _output_get (Variables|Default|SetInteraction%20Duration (Variables|/Game/Thomas/Interaction/InteractionArea/BP_InteractionArea_Master.BP_InteractionArea_Master_C|GetInteractionDuration (Variables|Default|GetFocusedInteractionArea))))
      (if (> _output_get 0.0)
        (bind _ref (Class|BIInteraction|InterfaceGetInteractionWidgetRef(Message) (Actor|GetParentActor (Variables|Default|GetFocusedInteractionArea))))
        (bind _aswb_interaction (Utilities|Casting|CastToWB_Interaction (UserInterface|GetWidget _ref)))
        (Variables|Default|SetCurrentInteractionWidgetREF _aswb_interaction)
        (bind _returnvalue (Utilities|Time|SetTimerbyEvent (delegate Custom|UpdateInteractionProgress) (Variables|Default|GetUpdateInteractionInterval) true))
        (Variables|Default|SetInteraction%20Timer _returnvalue)
        (else
          (CallFunction|UseInteract (Variables|Default|GetFocusedInteractionArea))
          (CallFunction|RunEventAfterInteraction))))
    (else
      (CallFunction|StopInteraction))))

(event Custom|UseInteract
  (params (Interaction%20Area :type BP%20Interaction%20Area%20Master%20Object%20Reference))
  (Class|BIInteraction|InterfaceInteract(Message) (Actor|GetParentActor Interaction%20Area)))

(event Custom|UpdateInteractionProgress
  (bind _output_get (Variables|Default|SetInteractionProgress (+ (Variables|Default|GetInteractionProgress) (* (/ 1.0 (Variables|Default|GetInteraction%20Duration)) (Variables|Default|GetUpdateInteractionInterval)))))
  (Default|SetPercent (Variables|Default|GetCurrentInteractionWidgetREF) _output_get)
  (if (>= (Variables|Default|GetInteractionProgress) 1.0)
    (CallFunction|StopInteraction)
    (CallFunction|UseInteract (Variables|Default|GetFocusedInteractionArea))
    (CallFunction|RunEventAfterInteraction)))

(event EventTick
  (params (DeltaSeconds :type Float%20%28single-precision%29))
  (CallFunction|Trace))

(fn Trace
  (bind _returnvalue (Game|GetPlayerCameraManager 0))
  (bind _returnvalue_2 (Transformation|GetActorLocation _returnvalue))
  (bind (_outhit _returnvalue_3) (Collision|LineTraceByChannel _returnvalue_2 (+ _returnvalue_2 (* (Math|Vector|GetForwardVector (Transformation|GetActorRotation _returnvalue)) (Variables|Default|GetTraceDistance))) "TraceTypeQuery1" false 0 "None"))
  (if _returnvalue_3
    (if (!= (Variables|Default|GetFocused%20Actor) (.HitActor (Collision|BreakHitResult _outhit)))
      (Variables|Default|SetFocused%20Actor (.HitActor (Collision|BreakHitResult _outhit)))
      (CallFunction|TraceInteractionArea (or (== (Utilities|GetClass (.HitActor (Collision|BreakHitResult _outhit))) "/Game/Thomas/Interaction/InteractionArea/BP_InteractionArea_Box.BP_InteractionArea_Box_C") (== (Utilities|GetClass (.HitActor (Collision|BreakHitResult _outhit))) "/Game/Thomas/Interaction/InteractionArea/BP_InteractionArea_CustomShape.BP_InteractionArea_CustomShape_C"))))
    (else
      (CallFunction|TraceInteractionArea false))))

(fn TraceInteractionArea
  (params (Trace :type Boolean))
  (if Trace
    (if (Variables|Default|GetIsTracingInteractionArea)
      (Default|ToggleFocus (Variables|Default|GetFocusedInteractionArea) false))
    (bind _asbp_interaction_area_master (Utilities|Casting|CastToBP_InteractionArea_Master (Variables|Default|GetFocused%20Actor)))
    (bind _output_get (Variables|Default|SetFocusedInteractionArea _asbp_interaction_area_master))
    (Default|ToggleFocus _output_get true)
    (Variables|Default|SetIsTracingInteractionArea true)
    (elif (Variables|Default|GetIsTracingInteractionArea)
      (Variables|Default|SetIsTracingInteractionArea false)
      (Default|ToggleFocus (Variables|Default|GetFocusedInteractionArea) false)
      (Variables|Default|SetFocused%20Actor 0)
      (Variables|Default|SetFocusedInteractionArea 0)
      (CallFunction|StopInteraction))))

(fn StopInteraction
  (if (> (Variables|Default|GetInteractionProgress) 0.0)
    (Utilities|Time|ClearandInvalidateTimerbyHandle (Variables|Default|GetInteraction%20Timer))
    (Utilities|IsValid (Variables|Default|GetCurrentInteractionWidgetREF)
      (:Is%20Valid
        (Default|SetPercent (Variables|Default|GetCurrentInteractionWidgetREF) 0.0)
        (Variables|Default|SetInteractionProgress 0.0)
        (Variables|Default|SetCurrentInteractionWidgetREF 0)))))

(fn RunEventAfterInteraction
  (bind _output_get (LocalVariables|SetParentActor (Actor|GetParentActor (Variables|Default|GetFocusedInteractionArea))))
  (if (== (Utilities|GetClass _output_get) "/Game/Thomas/Interaction/InteractableObjects/BP_TestBox.BP_TestBox_C")
    (Development|PrintString "TEST")))