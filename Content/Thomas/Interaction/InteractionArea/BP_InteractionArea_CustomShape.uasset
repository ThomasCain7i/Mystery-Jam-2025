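; Interaction area Blueprint whose shape is a custom static mesh, extending a parent interaction area class.
; The construction script assigns CustomShape to the Shape component, then runs the parent's construction script.
; With DEV enabled, every material slot shows the interaction trace debug material; otherwise the shape is hidden without affecting its children.
; The event graph holds no active logic.
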(event EventBeginPlay)

(event Collision|EventActorBeginOverlap
  (params (OtherActor :type Actor%20Object%20Reference)))

(event EventTick
  (params (DeltaSeconds :type Float%20%28single-precision%29)))

(fn ConstructionScript
  (Components|StaticMesh|SetStaticMesh (Variables|Default|GetShape) (Variables|Default|GetCustom%20Shape))
  (if (Variables|Default|GetDEV)
    (for _array_element (Class|MeshComponent|GetMaterialSlotNames (Variables|Default|GetShape))
      (Rendering|Material|SetMaterialbyName (Variables|Default|GetShape) _array_element "/Game/Thomas/Interaction/InteractionArea/M_InteractionTraceShape.M_InteractionTraceShape"))
    (else
      (Rendering|SetVisibility (Variables|Default|GetShape) false false)))
  (|CallParentFunction))