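; BP_PrideLightSwitch is an interactable switch in the Pride light-bulb puzzle, highlighting through custom depth on focus.
; Interacting plays a sound, toggles a fixed trio of five referenced bulbs chosen by SwitchNum, and animates the flip with a reversible timeline.
; After each toggle, CheckBulbs switches off a random bulb if all five are lit, so the all-on state never holds.
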(event Custom|UseInteract
  (Audio|PlaySound2D "/Game/Sounds/Pride/SC_Switch.SC_Switch" 1.0 1.0 0.0 0 0)
  (switch int (Variables|Default|GetSwitchNum)
    (:0
      (Default|TurnOn/Off (Variables|LightBulbs|GetLightBulb1)))
    (:1
      (Default|TurnOn/Off (Variables|LightBulbs|GetLightBulb1)))
    (:2
      (Default|TurnOn/Off (Variables|LightBulbs|GetLightBulb3)))
    (:3
      (Default|TurnOn/Off (Variables|LightBulbs|GetLightBulb1)))
    (:4
      (Default|TurnOn/Off (Variables|LightBulbs|GetLightBulb5))))
  (CallFunction|CheckBulbs)
  (if (Variables|Default|GetIsOn?)
    (bind _newtrack_0 (Timeline|Timeline ReverseFromEnd)
      (:Update
        (Transformation|SetRelativeRotation (Variables|Default|GetFlip) (Math|Rotator|MakeRotator (Math|Float|Lerp -45.0 45.0 _newtrack_0) 0.0 0.0) false false))
      (:Finished
        (Variables|Default|SetIsOn? (not (Variables|Default|GetIsOn?)))))
    (else
      (Timeline|Timeline PlayFromStart))))

(event Custom|Check%20Bulbs
  (if (Math|Boolean|ANDBoolean (Variables|/Game/Thomas/Interaction/InteractableObjects/Puzzle/Pride/BP_PrideLightBulb.BP_PrideLightBulb_C|GetIsOn? (Variables|LightBulbs|GetLightBulb1)) (Variables|/Game/Thomas/Interaction/InteractableObjects/Puzzle/Pride/BP_PrideLightBulb.BP_PrideLightBulb_C|GetIsOn? (Variables|LightBulbs|GetLightBulb2)) (Variables|/Game/Thomas/Interaction/InteractableObjects/Puzzle/Pride/BP_PrideLightBulb.BP_PrideLightBulb_C|GetIsOn? (Variables|LightBulbs|GetLightBulb3)) (Variables|/Game/Thomas/Interaction/InteractableObjects/Puzzle/Pride/BP_PrideLightBulb.BP_PrideLightBulb_C|GetIsOn? (Variables|LightBulbs|GetLightBulb4)) (Variables|/Game/Thomas/Interaction/InteractableObjects/Puzzle/Pride/BP_PrideLightBulb.BP_PrideLightBulb_C|GetIsOn? (Variables|LightBulbs|GetLightBulb5)))
    (switch int (Math|Random|RandomIntegerinRange 0 4)
      (:0
        (Default|TurnOn/Off (Variables|LightBulbs|GetLightBulb1)))
      (:1
        (Default|TurnOn/Off (Variables|LightBulbs|GetLightBulb2)))
      (:2
        (Default|TurnOn/Off (Variables|LightBulbs|GetLightBulb3)))
      (:3
        (Default|TurnOn/Off (Variables|LightBulbs|GetLightBulb4)))
      (:4
        (Default|TurnOn/Off (Variables|LightBulbs|GetLightBulb5))))))

(event EventInterfaceToggleFocus
  (params (Focus :type Boolean))
  (Rendering|SetRenderCustomDepth (Variables|Default|GetSwitch) Focus))

(event EventInterfaceInteract
  (CallFunction|UseInteract))

(fn ConstructionScript)

(fn InterfaceGetInteractionWidgetRef
  (return (Variables|Default|GetWidget)))