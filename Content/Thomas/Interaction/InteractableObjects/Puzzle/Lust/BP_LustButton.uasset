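; BP_LustButton is an interactable button for the Lust puzzle, acting as either the start button or a number button.
; Interacting with the start button starts the puzzle on BP_DisplayCase, while number buttons pass their Number to BP_LustPuzzle and update its latest number.
; Both targets are found with GetActorOfClass.
; Focus toggles a custom-depth highlight on the mesh, which cannot switch on once LustPuzzleComplete is set.
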(event Custom|UseInteract
  (if (Variables|Default|GetIsStartButton?)
    (bind _returnvalue (Actor|GetActorOfClass "/Game/Thomas/Puzzle/BP_DisplayCase.BP_DisplayCase_C"))
    (Default|StartPuzzle _returnvalue)
    (Variables|Default|SetLustPuzzleStarted true)
    (else
      (bind _returnvalue_2 (Actor|GetActorOfClass "/Game/Thomas/Puzzle/BP_LustPuzzle.BP_LustPuzzle_C"))
      (Variables|/Game/Thomas/Puzzle/BP_LustPuzzle.BP_LustPuzzle_C|SetSelectedNumber _returnvalue_2 (Variables|Default|GetNumber))
      (Default|UpdateLatestNumber _returnvalue_2))))

(event EventInterfaceToggleFocus
  (params (Focus :type Boolean))
  (if (not (and (Variables|Default|GetLustPuzzleComplete) Focus))
    (Rendering|SetRenderCustomDepth (Variables|Default|GetMesh%201) Focus)))

(event EventInterfaceInteract
  (CallFunction|UseInteract))

(fn ConstructionScript)

(fn InterfaceGetInteractionWidgetRef
  (return (Variables|Default|GetWidget)))