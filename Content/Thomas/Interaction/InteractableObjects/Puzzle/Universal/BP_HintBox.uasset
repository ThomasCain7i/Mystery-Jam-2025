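; BP_HintBox is an interactable puzzle prop that shows a room-specific hint on the player HUD.
; Through interaction interface events, focus toggles the cone's custom depth and, while no hint is active, shows or clears a warning text.
; Interacting raises a flag, writes the hint to the PlayerHUD widget found on focus, then clears the text and flag after a timed delay.
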(event Custom|UseInteract
  (Variables|Default|SetIsHintOn? true)
  (Variables|/Game/Thomas/UI/PlayerHUD.PlayerHUD_C|SetCurrentText (Variables|Default|GetPlayer%20HUD%20REF) (Variables|Default|GetRoomSpecificHint))
  (Utilities|FlowControl|Delay (Variables|Default|GetHint%20Timer))
  (Variables|/Game/Thomas/UI/PlayerHUD.PlayerHUD_C|SetCurrentText (Variables|Default|GetPlayer%20HUD%20REF) "")
  (Variables|Default|SetIsHintOn? false))

(event EventInterfaceToggleFocus
  (params (Focus :type Boolean))
  (Rendering|SetRenderCustomDepth (Variables|Default|GetCone) Focus)
  (if (and Focus (not (Variables|Default|GetIsHintOn?)))
    (bind _foundwidgets (Widget|GetAllWidgetsOfClass "/Game/Thomas/UI/PlayerHUD.PlayerHUD_C" false))
    (bind _output_get (Variables|Default|SetPlayer%20HUD%20REF (Utilities|Array|Get(acopy) _foundwidgets)))
    (Variables|/Game/Thomas/UI/PlayerHUD.PlayerHUD_C|SetCurrentText _output_get (Variables|Default|GetHint%20Warning%20Text))
    (elif (not (Variables|Default|GetIsHintOn?))
      (Variables|/Game/Thomas/UI/PlayerHUD.PlayerHUD_C|SetCurrentText _output_get ""))))

(event EventInterfaceInteract
  (CallFunction|UseInteract))

(fn ConstructionScript)

(fn InterfaceGetInteractionWidgetRef
  (return (Variables|Default|GetWidget)))