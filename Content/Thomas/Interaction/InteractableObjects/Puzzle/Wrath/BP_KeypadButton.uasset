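; BP_KeypadButton is a single clickable keypad button actor in the Wrath puzzle.
; It applies its configured number mesh on BeginPlay and swaps material to show cursor hover, with ResetButtons also restoring the default safe material.
; On click it passes its value and confirm/backspace flags to the referenced keypad actor through ButtonEntered, leaving input handling to that actor.
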(event OnBeginCursorOver(Button)
  (params (TouchedComponent :type Primitive%20Component%20Object%20Reference))
  (Rendering|Material|SetMaterial (Variables|Default|GetButton) 0 "/Game/Thomas/Puzzle/M_Black.M_Black"))

(event OnEndCursorOver(Button)
  (params (TouchedComponent :type Primitive%20Component%20Object%20Reference))
  (Rendering|Material|SetMaterial (Variables|Default|GetButton) 0 "/Game/R60D/Materials/M_Safe.M_Safe"))

(event OnClicked(Button)
  (params (TouchedComponent :type Primitive%20Component%20Object%20Reference) (ButtonPressed :type Key%20Structure))
  (Default|ButtonEntered (Variables|Default|GetKeypadActor%20REF) (Variables|Default|GetNumberText) (Variables|Default|GetConfirmedButton?) (Variables|Default|GetBackspaceButton?)))

(event Custom|Reset%20Buttons
  (Rendering|Material|SetMaterial (Variables|Default|GetButton) 0 "/Game/R60D/Materials/M_Safe.M_Safe"))

(event EventBeginPlay
  (Components|StaticMesh|SetStaticMesh (Variables|Default|GetButton) (Variables|Default|GetButtonNumberMesh)))

(fn ConstructionScript)

(fn InterfaceGetInteractionWidgetRef
  (return 0))