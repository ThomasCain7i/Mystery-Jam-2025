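; BP_Keypad is an interactable puzzle safe that opens when the player enters the correct code.
; Box overlap registers it with the player, focus toggles the door's custom-depth highlight, and interacting blends to the keypad camera with mouse clicking enabled.
; Child-actor BP_KeypadButtons feed input into a text display, which is compared to KeypadCode on confirm.
; Success restores player view and swings the door via timeline, notifying BP_GameManager for Envy safes; failure resets the buttons.
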(event OnComponentBeginOverlap(Box)
  (params (OverlappedComponent :type Primitive%20Component%20Object%20Reference) (OtherActor :type Actor%20Object%20Reference) (OtherComp :type Primitive%20Component%20Object%20Reference) (OtherBodyIndex :type Integer) (bFromSweep :type Boolean) (SweepResult :type Hit%20Result%20Structure%20%28by%20ref%29))
  (if (Actor|ActorHasTag OtherActor "Player")
    (bind _asbp_first_person_character (Utilities|Casting|CastToBP_FirstPersonCharacter OtherActor))
    (Variables|Default|SetPlayer%20REF _asbp_first_person_character)
    (Variables|/Game/FirstPerson/Blueprints/BP_FirstPersonCharacter.BP_FirstPersonCharacter_C|SetKeypadInteractActor _asbp_first_person_character self)))

(event OnComponentEndOverlap(Box)
  (params (OverlappedComponent :type Primitive%20Component%20Object%20Reference) (OtherActor :type Actor%20Object%20Reference) (OtherComp :type Primitive%20Component%20Object%20Reference) (OtherBodyIndex :type Integer))
  (if (Actor|ActorHasTag OtherActor "Player")
    (bind _asbp_first_person_character (Utilities|Casting|CastToBP_FirstPersonCharacter OtherActor))
    (Variables|/Game/FirstPerson/Blueprints/BP_FirstPersonCharacter.BP_FirstPersonCharacter_C|SetKeypadInteractActor _asbp_first_person_character 0)))

(event Custom|UseInteract
  (if (Variables|Default|GetIsInteracting?)
    (CallFunction|UnInteract)
    (elif (not (Variables|Default|GetSafeOpened?))
      (CallFunction|OnInteracted))))

(event Custom|On%20Interacted
  (bind _returnvalue (Game|GetPlayerController 0))
  (Variables|Default|SetIsInteracting? true)
  (Game|Player|SetViewTargetwithBlend (Game|GetPlayerController 0) (Components|GetOwner (Variables|Default|GetCamera)) 0.5 "VTBlend_Linear" 0.0 false)
  (bind _output_get (Variables|/Script/Engine.PlayerController|SetbShowMouseCursor _returnvalue true))
  (bind _output_get_2 (Variables|/Script/Engine.PlayerController|SetbEnableClickEvents _returnvalue _output_get))
  (Variables|/Script/Engine.PlayerController|SetbEnableMouseOverEvents _returnvalue _output_get_2)
  (bind _output_get_3 (Variables|Default|SetButtonsArray (Utilities|Array|MakeArray (Variables|Buttons|GetButton1) (Variables|Buttons|GetButton2) (Variables|Buttons|GetButton3) (Variables|Buttons|GetButton4) (Variables|Buttons|GetButton5) (Variables|Buttons|GetButton6) (Variables|Buttons|GetButton7) (Variables|Buttons|GetButton8) (Variables|Buttons|GetButton9) (Variables|Buttons|GetButton_Clear) (Variables|Buttons|GetButton0) (Variables|Buttons|GetButton_Enter))))
  (for _array_element _output_get_3
    (bind _asbp_keypad_button (Utilities|Casting|CastToBP_KeypadButton (Variables|/Script/Engine.ChildActorComponent|GetChildActor _array_element)))
    (Variables|/Game/Thomas/Interaction/InteractableObjects/Puzzle/Wrath/BP_KeypadButton.BP_KeypadButton_C|SetKeypadActor%20REF _asbp_keypad_button self)
    (CallFunction|ToggleFocus(UsingKeypad))))

(event Custom|Initiate
  (bind _returnvalue (Game|GetPlayerController 0))
  (bind _output_get (Variables|/Script/Engine.PlayerController|SetbShowMouseCursor _returnvalue true))
  (bind _output_get_2 (Variables|/Script/Engine.PlayerController|SetbEnableClickEvents _returnvalue _output_get))
  (Variables|/Script/Engine.PlayerController|SetbEnableMouseOverEvents _returnvalue _output_get_2)
  (bind _output_get_3 (Variables|Default|SetButtonsArray (Utilities|Array|MakeArray (Variables|Buttons|GetButton1) (Variables|Buttons|GetButton2) (Variables|Buttons|GetButton3) (Variables|Buttons|GetButton4) (Variables|Buttons|GetButton5) (Variables|Buttons|GetButton6) (Variables|Buttons|GetButton7) (Variables|Buttons|GetButton8) (Variables|Buttons|GetButton9) (Variables|Buttons|GetButton_Clear) (Variables|Buttons|GetButton0) (Variables|Buttons|GetButton_Enter))))
  (for _array_element _output_get_3
    (bind _asbp_keypad_button (Utilities|Casting|CastToBP_KeypadButton (Variables|/Script/Engine.ChildActorComponent|GetChildActor _array_element)))
    (Variables|/Game/Thomas/Interaction/InteractableObjects/Puzzle/Wrath/BP_KeypadButton.BP_KeypadButton_C|SetKeypadActor%20REF _asbp_keypad_button self)
    (CallFunction|ToggleFocus(UsingKeypad))))

(event Custom|Toggle%20Focus%20%28Using%20Keypad%29
  (Rendering|SetRenderCustomDepth (Variables|Default|GetSM_SafeDoor) (not (stale EventInterfaceToggleFocus Focus))))

(event Custom|Button%20Entered
  (params (Value :type Text) (Confirmed? :type Boolean) (Backspace :type Boolean))
  (bind _returnvalue (Utilities|String|ToString(Text) Value))
  (bind _enteredcode (Variables|Default|GetEnteredCode))
  (bind _text (Variables|/Script/Engine.TextRenderComponent|GetText _enteredcode))
  (bind _returnvalue_2 (Utilities|String|ToString(Text) _text))
  (bind _returnvalue_3 (Utilities|String|Append _returnvalue_2 _returnvalue))
  (bind _returnvalue_4 (Utilities|Text|ToText(String) _returnvalue_3))
  (Development|PrintString (Utilities|String|ToString(Text) _returnvalue_4))
  (if Confirmed?
    (CallFunction|Confirmed)
    (elif Backspace
      (CallFunction|Backspace)
      (elif (Variables|Default|GetCanEnter)
        (Rendering|Components|TextRender|SetText (Variables|Default|GetEnteredCode) (Utilities|Text|ToText(String) (Utilities|String|Replace (Utilities|String|ToString(Text) (Variables|/Script/Engine.TextRenderComponent|GetText (Variables|Default|GetEnteredCode))) (Utilities|String|GetSubstring (Utilities|String|MakeLiteralString "..........") 0 (Utilities|String|Len (Variables|Default|GetKeypad%20Code))))))
        (Rendering|Components|TextRender|SetText (Variables|Default|GetEnteredCode) _returnvalue_4)))))

(event Custom|Backspace
  (Rendering|Components|TextRender|SetText (Variables|Default|GetEnteredCode) (Utilities|Text|MakeLiteralText "")))

(event Custom|Confirmed
  (bind _returnvalue (Game|GetPlayerController 0))
  (bind _returnvalue_2 (Game|GetPlayerController 0))
  (bind _returnvalue_3 (Game|GetPlayerController 0))
  (if (Utilities|Enum|Equal(Enum) (Variables|Default|GetKeypad%20Code) (Utilities|String|ToString(Text) (Variables|/Script/Engine.TextRenderComponent|GetText (Variables|Default|GetEnteredCode))))
    (Utilities|FlowControl|Sequence
      (:then_0
        (Development|PrintString "Correct Passcode")
        (bind _output_get (Variables|/Script/Engine.PlayerController|SetbShowMouseCursor _returnvalue_3 false))
        (bind _output_get_2 (Variables|/Script/Engine.PlayerController|SetbEnableMouseOverEvents _returnvalue_3 _output_get))
        (Variables|/Script/Engine.PlayerController|SetbEnableClickEvents _returnvalue_3 _output_get_2)
        (for _array_element (Variables|Default|GetButtonsArray)
          (bind _asbp_keypad_button (Utilities|Casting|CastToBP_KeypadButton (Variables|/Script/Engine.ChildActorComponent|GetChildActor _array_element)))
          (Default|ResetButtons _asbp_keypad_button)
          (Variables|Default|SetSafeOpened? true))
        (Game|Player|SetViewTargetwithBlend _returnvalue_2 (Components|GetOwner (Variables|/Game/FirstPerson/Blueprints/BP_FirstPersonCharacter.BP_FirstPersonCharacter_C|GetFirstPersonCamera (.AsBP%20First%20Person%20Character (Utilities|Casting|CastToBP_FirstPersonCharacter (Game|Player|GetPlayerPawn 0))))) 0.5 "VTBlend_Linear" 0.0 false)
        (Input|SetInputModeGameOnly _returnvalue_2 false)
        (CallFunction|SafeOpened))
      (:then_1
        (Variables|Default|SetCanEnter false)))
    (else
      (Utilities|FlowControl|Sequence
        (:then_0
          (Development|PrintString "InCorrect Passcode")
          (bind _output_get_3 (Variables|/Script/Engine.PlayerController|SetbShowMouseCursor _returnvalue false))
          (bind _output_get_4 (Variables|/Script/Engine.PlayerController|SetbEnableMouseOverEvents _returnvalue _output_get_3))
          (Variables|/Script/Engine.PlayerController|SetbEnableClickEvents _returnvalue _output_get_4))
        (:then_1
          (Variables|Default|SetCanEnter false)
          (for _array_element_2 (Variables|Default|GetButtonsArray)
            (bind _asbp_keypad_button_2 (Utilities|Casting|CastToBP_KeypadButton (Variables|/Script/Engine.ChildActorComponent|GetChildActor _array_element_2)))
            (Default|ResetButtons _asbp_keypad_button_2))
          (CallFunction|Initiate)
          (Variables|Default|SetCanEnter true))))))

(event Custom|UnInteract
  (bind _returnvalue (Game|GetPlayerController 0))
  (bind _returnvalue_2 (Game|GetPlayerController 0))
  (bind _output_get (Variables|/Script/Engine.PlayerController|SetbShowMouseCursor _returnvalue false))
  (bind _output_get_2 (Variables|/Script/Engine.PlayerController|SetbEnableMouseOverEvents _returnvalue _output_get))
  (Variables|/Script/Engine.PlayerController|SetbEnableClickEvents _returnvalue _output_get_2)
  (Game|Player|SetViewTargetwithBlend _returnvalue_2 (Components|GetOwner (Variables|/Game/FirstPerson/Blueprints/BP_FirstPersonCharacter.BP_FirstPersonCharacter_C|GetFirstPersonCamera (.AsBP%20First%20Person%20Character (Utilities|Casting|CastToBP_FirstPersonCharacter (Game|Player|GetPlayerPawn 0))))) 0.5 "VTBlend_Linear" 0.0 false)
  (Input|SetInputModeGameOnly _returnvalue_2 false)
  (Variables|Default|SetIsInteracting? false))

(event Custom|SafeOpened
  (bind _newtrack_0 (Timeline|OpenSafeDoor Play)
    (:Update
      (Transformation|SetRelativeRotation (Variables|Default|GetSM_SafeDoor) (Math|Rotator|MakeRotator 0.0 0.0 (Math|Float|Lerp 9e+01 -35.0 _newtrack_0)) false false)
      (if (Variables|Default|GetEnvySafe?)
        (bind _returnvalue (Actor|GetActorOfClass "/Game/Thomas/Managers/BP_GameManager.BP_GameManager_C"))
        (Default|EnvyPuzzleComplete _returnvalue)))))

(event EventBeginPlay)

(event EventInterfaceToggleFocus
  (params (Focus :type Boolean))
  (Rendering|SetRenderCustomDepth (Variables|Default|GetSM_SafeDoor) Focus))

(event EventInterfaceInteract
  (CallFunction|UseInteract))

(fn ConstructionScript)

(fn InterfaceGetInteractionWidgetRef
  (return (Variables|Default|GetWidget)))