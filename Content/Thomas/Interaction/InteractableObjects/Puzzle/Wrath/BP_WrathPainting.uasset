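; BP_WrathPainting is an interactable painting, filed under the Wrath puzzle, whose frame tilts when used.
; Focus toggles custom depth rendering on the painting mesh, and the interaction interface exposes its widget.
; Interacting calls UseInteract, which plays a timeline that lerps the frame's relative pitch to a tilted angle, with no reverse path.
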(event Custom|UseInteract
  (bind _newtrack_0 (Timeline|Timeline Play)
    (:Update
      (Transformation|SetRelativeRotation (Variables|Default|GetFrame) (Math|Rotator|MakeRotator 0.0 (Math|Float|Lerp 0.0 -3e+01 _newtrack_0) 0.0) false false))))

(event EventBeginPlay)

(event EventInterfaceToggleFocus
  (params (Focus :type Boolean))
  (Rendering|SetRenderCustomDepth (Variables|Default|GetPainting) Focus))

(event EventInterfaceInteract
  (CallFunction|UseInteract))

(fn ConstructionScript)

(fn InterfaceGetInteractionWidgetRef
  (return (Variables|Default|GetWidget)))