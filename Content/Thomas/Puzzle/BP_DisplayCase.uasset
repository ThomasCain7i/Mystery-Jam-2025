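; BP_DisplayCase is a puzzle display that flashes a fixed sequence of item images (spray paint, bleach, scissors) on its Screen.
; StartPuzzle runs only if the previous display has finished and the puzzle is incomplete.
; It chains Change Screen Display calls, each swapping the material, showing it for a delay, then hiding it.
; When the sequence ends, it finds BP_LustPuzzle by class and sets its PuzzleStarted flag.
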(event Custom|Start%20Puzzle
  (if (and (Variables|Default|GetDisplayFinished) (not (Variables|Default|GetPuzzleComplete)))
    (Variables|Default|SetDisplayFinished false)
    (Utilities|FlowControl|Delay 1.0)
    (Development|PrintString "Puzzle Started")
    (Rendering|SetVisibility (Variables|Default|GetScreen) true false)
    (Variables|Default|SetPuzzleStarted true)
    (Utilities|ChangeScreenDisplay (Variables|Default|GetSpray%20Paint%20M)
      (:Output
        (Utilities|ChangeScreenDisplay (Variables|Default|GetBleach%20M)
          (:Output
            (Utilities|ChangeScreenDisplay (Variables|Default|GetScissors%20M)
              (:Output
                (Utilities|ChangeScreenDisplay (Variables|Default|GetBleach%20M)
                  (:Output
                    (Utilities|ChangeScreenDisplay (Variables|Default|GetSpray%20Paint%20M)
                      (:Output
                        (Variables|Default|SetDisplayFinished true)
                        (bind _returnvalue (Actor|GetActorOfClass "/Game/Thomas/Puzzle/BP_LustPuzzle.BP_LustPuzzle_C"))
                        (Variables|/Game/Thomas/Puzzle/BP_LustPuzzle.BP_LustPuzzle_C|SetPuzzleStarted _returnvalue true)))))))))))))

(fn ConstructionScript)