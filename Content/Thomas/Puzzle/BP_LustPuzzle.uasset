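; Lust puzzle controller that checks a five-number input sequence against a fixed answer.
; While the puzzle is running, each UpdateLatestNumber call stores SelectedNumber in the next slot, and the fifth triggers the check.
; Success flags every BP_LustButton and the display case, notifies BP_GameManager, restores LustPainting and plays a sound.
; Failure clears the sequence, restarts the puzzle through BP_DisplayCase, corrupts the painting and plays an error sound.
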(event Custom|UpdateLatestNumber
  (if (and (not (Variables|Default|GetPuzzle%20Complete)) (Variables|Default|GetPuzzleStarted))
    (if (== (Variables|Default|GetCurrentSequence) 0)
      (Variables|Sequence|SetSequence1 (Variables|Default|GetSelectedNumber))
      (Development|PrintString (Utilities|String|ToString(Integer) (Variables|Sequence|GetSequence1)) true true "(R=0.000000,G=0.660000,B=1.000000,A=1.000000)" 1.0 :!label _label)
      (bind _result (Math|Integer|IncrementInt (Variables|Default|GetCurrentSequence))
        (:%20%20
          (Variables|Default|SetCurrentSequence _result)))
      (elif (== (Variables|Default|GetCurrentSequence) 1)
        (Variables|Sequence|SetSequence2 (Variables|Default|GetSelectedNumber))
        (Development|PrintString (Utilities|String|ToString(Integer) (Variables|Sequence|GetSequence2)) true true "(R=0.000000,G=0.660000,B=1.000000,A=1.000000)" 1.0 :!label _label_2)
        (goto _label)
        (elif (== (Variables|Default|GetCurrentSequence) 2)
          (Variables|Sequence|SetSequence3 (Variables|Default|GetSelectedNumber))
          (Development|PrintString (Utilities|String|ToString(Integer) (Variables|Sequence|GetSequence3)) true true "(R=0.000000,G=0.660000,B=1.000000,A=1.000000)" 1.0 :!label _label_3)
          (goto _label_2)
          (elif (== (Variables|Default|GetCurrentSequence) 3)
            (Variables|Sequence|SetSequence4 (Variables|Default|GetSelectedNumber))
            (Development|PrintString (Utilities|String|ToString(Integer) (Variables|Sequence|GetSequence4)) true true "(R=0.000000,G=0.660000,B=1.000000,A=1.000000)" 1.0)
            (goto _label_3)
            (elif (== (Variables|Default|GetCurrentSequence) 4)
              (Variables|Sequence|SetSequence5 (Variables|Default|GetSelectedNumber))
              (Variables|Default|SetCurrentSequence 0)
              (CallFunction|CheckAnswer))))))))

(event Custom|CheckAnswer
  (if (Math|Boolean|ANDBoolean (== (Variables|Sequence|GetSequence1) 1) (== (Variables|Sequence|GetSequence2) 2) (== (Variables|Sequence|GetSequence3) 3) (== (Variables|Sequence|GetSequence4) 2) (== (Variables|Sequence|GetSequence5) 1))
    (Development|PrintString "PUZZLE COMPLETE")
    (bind _outactors (Actor|GetAllActorsOfClass "/Game/Thomas/Interaction/InteractableObjects/Puzzle/Lust/BP_LustButton.BP_LustButton_C"))
    (for _array_element _outactors
      (Variables|/Game/Thomas/Interaction/InteractableObjects/Puzzle/Lust/BP_LustButton.BP_LustButton_C|SetLustPuzzleComplete _array_element true)
      (bind _returnvalue (Actor|GetActorOfClass "/Game/Thomas/Puzzle/BP_DisplayCase.BP_DisplayCase_C"))
      (Variables|/Game/Thomas/Puzzle/BP_DisplayCase.BP_DisplayCase_C|SetPuzzleComplete _returnvalue true)
      (Default|LustPuzzleComplete (Variables|Default|GetGameManager))
      ;[1 1 1] This will set the painting to normal
      (Default|SetPainting (Variables|Default|GetLustPainting) 0.0)
      (Audio|PlaySound2D "/Game/Sounds/Lust/Correct.Correct" 1.0 1.0 0.0 0 0))
    (else
      (CallFunction|ResetPuzzle)
      ;[1 1 1] This will corrupt the painting
      (Default|SetPainting (Variables|Default|GetLustPainting) 1.0)
      (Audio|PlaySound2D "/Game/Sounds/Lust/Wrong.Wrong" 1.0 1.0 0.0 0 0))))

(event Custom|Reset%20Puzzle
  (Variables|Sequence|SetSequence1 0)
  (Variables|Sequence|SetSequence2 0)
  (Variables|Sequence|SetSequence3 0)
  (Variables|Sequence|SetSequence4 0)
  (Variables|Sequence|SetSequence5 0)
  (Variables|Default|SetCurrentSequence 0)
  (Development|PrintString "PUZZLE FAILED")
  (bind _returnvalue (Actor|GetActorOfClass "/Game/Thomas/Puzzle/BP_DisplayCase.BP_DisplayCase_C"))
  (Default|StartPuzzle _returnvalue))

(event EventBeginPlay
  (bind _returnvalue (Actor|GetActorOfClass "/Game/Thomas/Managers/BP_GameManager.BP_GameManager_C"))
  (Variables|Default|SetGameManager _returnvalue))

(fn ConstructionScript)