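; BP_WrathStatue3 is a pickup statue item for the Wrath puzzle that the player can focus on and interact with.
; On BeginPlay, its interact-with-item component sets up the item mesh data, and focus toggles the mesh's custom depth.
; Interacting picks up the item, increments the statue count on the BP_WrathManager found via GetActorOfClass, then destroys the actor.
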(event Custom|UseInteract
  (Default|PickUpItem (Variables|Default|GetBPC_InteractWithItem))
  (bind _returnvalue (Actor|GetActorOfClass "/Game/Thomas/Managers/BP_WrathManager.BP_WrathManager_C"))
  (Default|IncreaseStatueCount _returnvalue)
  (Actor|DestroyActor))

(event EventBeginPlay
  (Default|SetUpItemMeshData (Variables|Default|GetBPC_InteractWithItem) (Variables|/Script/Engine.StaticMeshComponent|GetStaticMesh (Variables|Default|GetItem))))

(event EventInterfaceInteract
  (CallFunction|UseInteract))

(event EventInterfaceToggleFocus
  (params (Focus :type Boolean))
  (Rendering|SetRenderCustomDepth (Variables|Default|GetItem) Focus))

(fn ConstructionScript)

(fn InterfaceGetInteractionWidgetRef
  (return (Variables|Default|GetWidget)))