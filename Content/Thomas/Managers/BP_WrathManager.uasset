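; BP_WrathManager tracks collected statues and reveals a statue once all six are gathered.
; It responds to interaction interface events, highlighting a cone mesh through custom depth on focus and exposing its widget reference.
; An external call increments the count, and interacting makes the statue visible only when the count reaches six.
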(event Custom|UseInteract
  (if (== (Variables|Default|GetStatuesCollected) 6)
    (Rendering|SetVisibility (Variables|Default|GetStatue) true false)))

(event Custom|IncreaseStatueCount
  (Variables|Default|SetStatuesCollected (+ (Variables|Default|GetStatuesCollected) 1)))

(event EventInterfaceInteract
  (CallFunction|UseInteract))

(event EventInterfaceToggleFocus
  (params (Focus :type Boolean))
  (Rendering|SetRenderCustomDepth (Variables|Default|GetCone) Focus))

(fn ConstructionScript)

(fn InterfaceGetInteractionWidgetRef
  (return (Variables|Default|GetWidget)))