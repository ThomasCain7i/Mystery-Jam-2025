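; BP_Door is a puzzle-room door that closes behind the player and tracks which of seven sin-themed rooms is active.
; A Timeline lerps the door's yaw to open and reverses to close; OpenDoor has no caller here.
; The InRoom overlap closes the door, latches PuzzleStarted and sets the BP_GameManager flag matching CurrentRoomNumber.
; Once started, the OutRoom overlap closes the door and clears the sin flags.
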(event OnComponentBeginOverlap(InRoom)
  (params (OverlappedComponent :type Primitive%20Component%20Object%20Reference) (OtherActor :type Actor%20Object%20Reference) (OtherComp :type Primitive%20Component%20Object%20Reference) (OtherBodyIndex :type Integer) (bFromSweep :type Boolean) (SweepResult :type Hit%20Result%20Structure%20%28by%20ref%29))
  (Development|PrintString (Utilities|String|ToString(Text) (Utilities|Text|FormatText "Entered {room number}" (Variables|Default|GetCurrentRoomNumber))))
  (if (and (Actor|ActorHasTag OtherActor "Player") (not (Variables|Default|GetPuzzle%20Started?)))
    (CallFunction|CloseDoor)
    (Variables|Default|SetPuzzle%20Started? true)
    (|IntSwitchCurrentRoom)))

(event OnComponentBeginOverlap(OutRoom)
  (params (OverlappedComponent :type Primitive%20Component%20Object%20Reference) (OtherActor :type Actor%20Object%20Reference) (OtherComp :type Primitive%20Component%20Object%20Reference) (OtherBodyIndex :type Integer) (bFromSweep :type Boolean) (SweepResult :type Hit%20Result%20Structure%20%28by%20ref%29))
  (Development|PrintString "Exited Room")
  (if (and (Actor|ActorHasTag OtherActor "Player") (Variables|Default|GetPuzzle%20Started?))
    (CallFunction|CloseDoor)
    (Utilities|NoCurrentRoom)))

(event Custom|OpenDoor
  (bind _open_door (Timeline|Timeline Play)
    (:Update
      (Transformation|SetRelativeRotation (Variables|Default|GetDoor) (Math|Rotator|MakeRotator 0.0 0.0 (Math|Float|Lerp (Variables|Default|GetClosed%20Rotation) (Variables|Default|GetOpen%20Rotation) _open_door)) false false))))

(event Custom|Close%20Door
  (bind _open_door (Timeline|Timeline Reverse)
    (:Update
      (Transformation|SetRelativeRotation (Variables|Default|GetDoor) (Math|Rotator|MakeRotator 0.0 0.0 (Math|Float|Lerp (Variables|Default|GetClosed%20Rotation) (Variables|Default|GetOpen%20Rotation) _open_door)) false false))))

(event EventBeginPlay
  (bind _returnvalue (Actor|GetActorOfClass "/Game/Thomas/Managers/BP_GameManager.BP_GameManager_C"))
  (Variables|Default|SetGame%20Manager%20REF _returnvalue))

(fn ConstructionScript)