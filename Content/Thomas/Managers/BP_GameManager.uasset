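; Game manager that tracks progression through seven deadly-sin puzzle rooms, starting play by opening the Lust door.
; Each puzzle-complete event sets its flag and calls OpenDoor on its own door, with Lust through Greed also opening the next sin's door.
; All but Sloth light their pedestal fire and play the completion sound.
; Envy opens no further door, and Sloth plays the game-complete sound instead.
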(event Custom|Greed%20Puzzle%20Complete
  (Variables|CompltetedPuzzleBools|SetGreedComplete? true)
  (Default|OpenDoor (Variables|Doors|GetGreedDoor))
  (Default|OpenDoor (Variables|Doors|GetEnvyDoor))
  ;[1 1 1] Activate Pedestal Fire
  (Default|ActivateFire (Variables|FinalPedestals|GetGreedPedestal))
  ;[1 0.6784 0.3451] Play sound
  (CallFunction|PlayPuzzleCompleteSound))

(event Custom|Lust%20Puzzle%20Complete
  (Variables|CompltetedPuzzleBools|SetLustComplete? true)
  (Default|OpenDoor (Variables|Doors|GetLustDoor))
  (Default|OpenDoor (Variables|Doors|GetGluttonyDoor))
  ;[1 1 1] Activate Pedestal Fire
  (Default|ActivateFire (Variables|FinalPedestals|GetLustPedestal))
  ;[1 0.6784 0.3451] Play sound
  (CallFunction|PlayPuzzleCompleteSound))

(event Custom|Envy%20Puzzle%20Complete
  (Variables|CompltetedPuzzleBools|SetEnvyComplete? true)
  (Default|OpenDoor (Variables|Doors|GetEnvyDoor))
  ;[1 1 1] Activate Pedestal Fire
  (Default|ActivateFire (Variables|FinalPedestals|GetEnvyPedestal))
  ;[1 0.6784 0.3451] Play sound
  (CallFunction|PlayPuzzleCompleteSound))

(event Custom|PlayPuzzleCompleteSound
  ;[1 0.6784 0.3451] Sounds
  (Audio|PlaySoundatLocation (Variables|Default|GetPuzzleCompleteSound) (Variables|Default|GetPuzzleCompleteSoundLocaiton) "0, 0, 0" 1.0 1.0 0.0 0 0 0 0))

(event Custom|Gluttony%20Puzzle%20Complete
  (Variables|CompltetedPuzzleBools|SetGluttonyComplete? true)
  (Default|OpenDoor (Variables|Doors|GetGluttonyDoor))
  (Default|OpenDoor (Variables|Doors|GetWrathDoor))
  ;[1 1 1] Activate Pedestal Fire
  (Default|ActivateFire (Variables|FinalPedestals|GetGluttonyPedestal))
  ;[1 0.6784 0.3451] Play sound
  (CallFunction|PlayPuzzleCompleteSound))

(event Custom|Play%20Final%20Sound
  ;[1 0.6784 0.3451] Sounds
  (Audio|PlaySoundatLocation (Variables|Default|GetGameCompleteSound) (Variables|Default|GetPuzzleCompleteSoundLocaiton) "0, 0, 0" 1.0 1.0 0.0 0 0 0 0))

(event Custom|Wrath%20Puzzle%20Complete
  (Variables|CompltetedPuzzleBools|SetWrathComplete? true)
  (Default|OpenDoor (Variables|Doors|GetWrathDoor))
  (Default|OpenDoor (Variables|Doors|GetPrideDoor))
  ;[1 1 1] Activate Pedestal Fire
  (Default|ActivateFire (Variables|FinalPedestals|GetWrathPedestal))
  ;[1 0.6784 0.3451] Play sound
  (CallFunction|PlayPuzzleCompleteSound))

(event Custom|Pride%20Puzzle%20Complete
  (Variables|CompltetedPuzzleBools|SetPrideComplete? true)
  (Default|OpenDoor (Variables|Doors|GetPrideDoor))
  (Default|OpenDoor (Variables|Doors|GetGreedDoor))
  ;[1 1 1] Activate Pedestal Fire
  (Default|ActivateFire (Variables|FinalPedestals|GetPridePedestal))
  ;[1 0.6784 0.3451] Play sound
  (CallFunction|PlayPuzzleCompleteSound))

(event Custom|Sloth%20Puzzle%20Complete
  (Variables|CompltetedPuzzleBools|SetSlothComplete? true)
  (Default|OpenDoor (Variables|Doors|GetSlothDoor))
  ;[1 0.6784 0.3451] Play sound
  (CallFunction|PlayFinalSound))

(event EventBeginPlay
  (Default|OpenDoor (Variables|Doors|GetLustDoor)))

(fn ConstructionScript)